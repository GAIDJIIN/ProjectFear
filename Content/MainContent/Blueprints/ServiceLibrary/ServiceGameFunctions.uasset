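; Blueprint function library of physics and collision helpers for gameplay code.
; One function pushes a hit, physics-simulating component or bone at the impact point along the trace direction, scaled by a given strength.
; The other runs a stationary box trace at a static mesh's bounds center, sized from unscaled local bounds with caller-supplied rotation.
; That trace always uses the Visibility channel, ignoring its TraceChannel input.
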(fn `MakeImpulseAtImpactLocation`
  (params (Hit :type "HitResult Structure (by ref)") (ImpulseStrength :type "Float (double-precision)" :default 1000.0) (__WorldContext :type "Object Object Reference"))
  (bind (_bblockinghit _binitialoverlap _time _distance _location _impactpoint _normal _impactnormal _physmat _hitactor _hitcomponent _hitbonename) (`GameplayStatics.BreakHitResult` Hit))
  (bind (_bblockinghit_2 _binitialoverlap_2 _time_2 _distance_2 _location_2 _impactpoint_2 _normal_2 _impactnormal_2 _physmat_2 _hitactor_2 _hitcomponent_2 _hitbonename_2 _bonename _hititem _elementindex _faceindex _tracestart _traceend) (`GameplayStatics.BreakHitResult` (`local.Hit`)))
  (bind (_bblockinghit_3 _binitialoverlap_3 _time_3 _distance_3 _location_3 _impactpoint_3 _normal_3 _impactnormal_3 _physmat_3 _hitactor_3 _hitcomponent_3 _hitbonename_3) (`GameplayStatics.BreakHitResult` (`local.Hit`)))
  (if _bblockinghit
    (`/Engine/EditorBlueprintResources/StandardMacros.IsValid` _hitcomponent
      (:`Is Valid`
        (if (`SceneComponent.IsSimulatingPhysics` _hitcomponent _hitbonename)
          (`PrimitiveComponent.AddImpulseAtLocation` _hitcomponent_3 (* (`KismetMathLibrary.GetForwardVector` (`KismetMathLibrary.FindLookAtRotation` _tracestart _traceend)) (`local.ImpulseStrength`)) _impactpoint_3 _hitbonename_3))))))

(fn `MakeStaticMeshBoxTrace`
  (params (StaticMesh :type "StaticMeshComponent Object Reference") (TraceRotation :type "Rotator Structure") (IgnoreActors :type "Array of Actor Object Reference") (`Trace Channel` :type "ETraceTypeQuery Enum" :default "TraceTypeQuery1") (DrawDebugTrace :type "EDrawDebugTrace Enum" :default "None") (DrawDebugTime :type "Float (double-precision)" :default 10.0))
  (returns (OutHit :type "HitResult Structure") (bHit :type Boolean))
  (locals (BoxCenterPoint :type "Vector Structure") (HalfSize :type "Vector Structure"))
  (bind (_min _max) (`StaticMeshComponent.GetLocalBounds` StaticMesh))
  (bind _boxcenterpoint (`local.BoxCenterPoint`))
  (set `local.BoxCenterPoint` (`KismetSystemLibrary.GetComponentBounds` StaticMesh))
  (set `local.HalfSize` (/ (`KismetMathLibrary.MakeVector` (`KismetMathLibrary.Abs` (- (.x _max) (.x _min))) (`KismetMathLibrary.Abs` (- (.y _max) (.y _min))) (`KismetMathLibrary.Abs` (- (.z _max) (.z _min)))) 2.0))
  (bind (_outhit _returnvalue) (`KismetSystemLibrary.BoxTraceSingle` null _boxcenterpoint _boxcenterpoint (`local.HalfSize`) (`local.TraceRotation`) "TraceTypeQuery1" false (`local.IgnoreActors`) (`local.DrawDebugTrace`) true (struct :`R` 0.942869 :`G` 1.0 :`B` 0.905673 :`A` 1.0) (struct :`R` 1.0 :`G` 0.066208 :`A` 1.0) (`local.DrawDebugTime`)))
  (return _outhit _returnvalue))