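; ServiceMathFunctions is a Blueprint function library of small, stateless helpers for comparisons, array indices and rotators.
; It tests data table row handles for equality by table and row name, and pairs an array Find with a found flag.
; Index helpers clamp to an array's bounds or wrap by modulo, mirroring negatives from the end.
; Rotator helpers add and divide component by component, without quaternion composition or angle normalization.
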(fn `AddRotator`
  (params (Rotator1 :type "Rotator Structure") (Rotator2 :type "Rotator Structure"))
  (returns (ReturnValue :type "Rotator Structure"))
  (return (`KismetMathLibrary.MakeRotator` (+ (.roll Rotator1) (.roll Rotator2)) (+ (.pitch Rotator1) (.pitch Rotator2)) (+ (.yaw Rotator1) (.yaw Rotator2)))))

(fn `DivideRotator`
  (params (Rotator :type "Rotator Structure") (Divider :type "Float (double-precision)"))
  (returns (DividedRotator :type "Rotator Structure"))
  (bind _divider (`local.Divider`))
  (return (`KismetMathLibrary.MakeRotator` (/ (.roll Rotator) _divider) (/ (.pitch Rotator) _divider) (/ (.yaw Rotator) _divider))))

(fn `EqualDataTableRowHandle`
  (params (DataTableRowHandle1 :type "DataTableRowHandle Structure (by ref)") (DataTableRowHandle2 :type "DataTableRowHandle Structure (by ref)"))
  (returns (ReturnValue :type Boolean))
  (bind (_datatable _rowname) (break `DataTableRowHandle` DataTableRowHandle1))
  (bind (_datatable_2 _rowname_2) (break `DataTableRowHandle` DataTableRowHandle2))
  (return (and (== _datatable _datatable_2) (== _rowname _rowname_2))))

(fn `FindItemWithBool`
  (params (TargetArray :type "Array of Object Object Reference") (Item :type "Object Object Reference"))
  (returns (`IsFind?` :type Boolean) (SlotIndex :type Integer))
  (bind _returnvalue (`KismetArrayLibrary.Array_Find` TargetArray Item))
  (return (!= _returnvalue -1) _returnvalue))

(fn `GetClampedIndexFromArray`
  (params (IndexToClamp :type Integer) (TargetArray :type "Array of Object Object Reference"))
  (returns (ClampedIndex :type Integer))
  (return (`KismetMathLibrary.Clamp` IndexToClamp 0 (- (`KismetArrayLibrary.Array_Length` TargetArray) 1))))

(fn `WrapArrayIndex`
  (params (Index :type Integer) (ArrayLength :type Integer))
  (returns (`Return Value` :type Integer))
  (return (`KismetMathLibrary.SelectInt` (- (`local.ArrayLength`) (mod (`KismetMathLibrary.Abs_Int` Index) ArrayLength)) (mod Index ArrayLength) (< Index 0))))