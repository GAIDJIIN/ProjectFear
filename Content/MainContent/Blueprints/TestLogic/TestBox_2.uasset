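; TestBox_2 is a test Blueprint with a StaticMesh component, holding debug logic for inspecting that mesh's local bounds.
; An unconnected chain prints the bounds' Min and Max, draws debug spheres at both corners and prints the distance between them.
; The spheres use local-space corners directly, without conversion to world space.
; BeginPlay and the Construction Script are empty, so none of this logic runs.
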(event `self.ReceiveBeginPlay`)

(fn `UserConstructionScript`)