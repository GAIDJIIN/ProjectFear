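; BP_Door is an interactable door that opens only when the player's backpack holds the item matching its KeyID.
; Interacting with the Door component plays the TimeDoor timeline to rotate it on yaw with an open sound, or plays MetalDoor_Close if the key is missing.
; Ending overlap with the Box reverses the timeline after a short delay, clearing the Open flag once the door finishes closing.
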(event `/Game/MainContent/Blueprints/Items/Interfaces/BPI_Interact.StartInteract`
  (params (Player :type "/Game/MainContent/Blueprints/Player/PlayerCore/BP_Player Object Reference") (HitComponent :type "PrimitiveComponent Object Reference"))
  (bind _returnvalue (`self.K2_GetActorLocation`))
  (if (== HitComponent (`self.Door`))
    (bind _success (`/Game/MainContent/Blueprints/Player/Components/Inventory/BPC_Inventory.FindItemByID` (`/Game/MainContent/Blueprints/Player/PlayerCore/BP_Player.Backpack` Player) (`self.KeyID`)))
    (if _success
      (if (not (`self.Open?`))
        (set `self.Open?` true)
        (`GameplayStatics.PlaySoundAtLocation` "/Game/MainContent/Blueprints/TestLogic/Door/Sounds/MetalDoor_Open.MetalDoor_Open" _returnvalue (struct) 1.0 1.0 0.0 null null null null)
        (bind (_direction _opendoor) (`Timeline|TimeDoor` :!label _label)
          (:`Update`
            (`SceneComponent.K2_SetRelativeRotation` (`self.Door`) (`KismetMathLibrary.MakeRotator` 0.0 0.0 _opendoor) false false))
          (:`Finished`
            (switch `ETimelineDirection` _direction
              (:`Backward`
                (`GameplayStatics.PlaySoundAtLocation` null (`self.K2_GetActorLocation`) (struct) 1.0 1.0 0.0 null null null null)
                (set `self.Open?` false))))))
      (else
        (`GameplayStatics.PlaySoundAtLocation` "/Game/MainContent/Blueprints/TestLogic/Door/Sounds/MetalDoor_Close.MetalDoor_Close" _returnvalue (struct) 1.0 1.0 0.0 null null null null)))))

(event `self.Box.OnComponentEndOverlap`
  (params (OverlappedComponent :type "PrimitiveComponent Object Reference") (OtherActor :type "Actor Object Reference") (OtherComp :type "PrimitiveComponent Object Reference") (OtherBodyIndex :type Integer))
  (`KismetSystemLibrary.Delay` 1.0)
  (if (`self.Open?`)
    (goto _label :!via `Reverse`)))

(fn `UserConstructionScript`)