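; Player character Blueprint handling movement, camera, crosshair widget and input for inventory and item use.
; Backpack component handles inventory, interaction and slots; EquipItem spawns the item's actor on a mesh socket chosen by item type.
; State-check macros gate interact, drop, use and reload, forwarding use and reload to the held item.
; Work in progress: debug prints, test keys, and a timed screen-center interaction trace whose result is unused.
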(event `EquipItem`
  (params (ItemObject :type "/Game/MainContent/Blueprints/Items/ItemObjectForInventory/BP_ItemObjectCore Object Reference"))
  (bind ((`EquipItemClass_51_E3D0B3EC41DC869E4E07A5B343C5A2E3` _equipitemclass) (`ItemType_23_3939123540436897D2B7FB99C9705EA9` _itemtype)) (break `/Game/MainContent/Blueprints/Player/Components/Inventory/S_Item` (`/Game/MainContent/Blueprints/Items/ItemObjectForInventory/BP_ItemObjectCore.GetItemStructure` ItemObject)))
  ;[1 1 1] Test_OperationsWithItem
  (bind _returnvalue (`|SpawnActorFromClass` _equipitemclass (`KismetMathLibrary.MakeTransform` (0.0 0.0 0.0)) "Undefined" "OverrideRootScale" null self ItemObject self))
  (set `self.CurrentItem` _returnvalue)
  (set `self.ItemInHand` _itemtype)
  (`self.K2_AttachToComponent` (`self.CurrentItem`) (`self.Mesh`) (`BlueprintMapLibrary.Map_Find` (`self.ItemSocketSpawn`) (`self.ItemInHand`)) "SnapToTarget" "SnapToTarget" "SnapToTarget" true))

(event `UnEquipItem`
  ;[1 1 1] Test_OperationsWithItem
  (set `self.ItemInHand` "NewEnumerator6")
  (`self.K2_DestroyActor` (`self.CurrentItem`)))

(event `self.ReceiveBeginPlay`
  ;[1 1 1] Взять оружие
  (bind _returnvalue (`|CreateWidget` "/Game/MainContent/Blueprints/TestLogic/W_AIM.W_AIM_C" (`GameplayStatics.GetPlayerController` 0)))
  (`UserWidget.AddToViewport` _returnvalue 0)
  (`/Game/MainContent/Blueprints/Player/Components/Inventory/BPC_Inventory.Initialize Owner` (`self.Backpack`) self)
  (`self.StartInteract`))

(event `StartInteract`
  ;[1 1 1] Взять оружие
  (bind _returnvalue (`KismetSystemLibrary.K2_SetTimer` null "IsInteractable?" 0.1 true))
  (set `self.InteractTimer` _returnvalue)
  (`KismetSystemLibrary.PrintString` "Interact"))

(event `StopInteract`
  ;[1 1 1] Взять оружие
  (`KismetSystemLibrary.K2_ClearAndInvalidateTimerHandle` (`self.InteractTimer`))
  (`KismetSystemLibrary.PrintString` "No Interact"))

(event `InputAction|Inventory`
  (params (Key :type "Key Structure"))
  ;[1 1 1] Input
  (:`Pressed`
    (`/Game/MainContent/Blueprints/Player/Components/Inventory/BPC_Inventory.ToggleInventory` (`self.Backpack`) Key)))

(event `InputAxis|MoveForward`
  (params (AxisValue :type "Float (single-precision)"))
  ;[1 1 1] Input
  (bind _output_get (set `self.AxisForward` AxisValue))
  (`self.MoveForward` _output_get (!= _output_get 0.0)))

(event `InputAxis|LookUD`
  (params (AxisValue :type "Float (single-precision)"))
  ;[1 1 1] Input
  (bind _output_get (set `self.AxisLookUD` AxisValue))
  (`self.AddControllerPitchInput` _output_get))

(event `InputAction|FirstWeapon`
  (params (Key :type "Key Structure"))
  ;[1 1 1] Equip&UnEquip Items
  (:`Pressed`
    (`/Game/MainContent/Blueprints/Player/Components/Inventory/BPC_Inventory.EquipWeapon` (`self.Backpack`) 0)))

(event `Key|Three`
  (params (Key :type "Key Structure"))
  ;[1 1 1] Equip&UnEquip Items
  (:`Pressed`
    (`/Game/MainContent/Blueprints/Player/Components/Inventory/BPC_Inventory.Test_EquipItemFromFastSlot` (`self.Backpack`) 0)))

(event `InputAction|SecondWeapon`
  (params (Key :type "Key Structure"))
  ;[1 1 1] Equip&UnEquip Items
  (:`Pressed`
    (`/Game/MainContent/Blueprints/Player/Components/Inventory/BPC_Inventory.EquipWeapon` (`self.Backpack`) 1)))

(event `InputAxis|MoveRight`
  (params (AxisValue :type "Float (single-precision)"))
  ;[1 1 1] Input
  (bind _output_get (set `self.AxisRight` AxisValue))
  (`self.MoveRight` _output_get (!= _output_get 0.0)))

(event `InputAxis|LookLR`
  (params (AxisValue :type "Float (single-precision)"))
  ;[1 1 1] Input
  (bind _output_get (set `self.AxisLookLR` AxisValue))
  (`self.AddControllerYawInput` _output_get))

(event `InputAction|Interact`
  (params (Key :type "Key Structure"))
  ;[1 1 1] Input
  (:`Pressed`
    (`self.CanInteract?`
      (:`finish`
        (`/Game/MainContent/Blueprints/Player/Components/Inventory/BPC_Inventory.Interact` (`self.Backpack`))))))

(event `Key|Four`
  (params (Key :type "Key Structure"))
  ;[1 1 1] Equip&UnEquip Items
  (:`Pressed`
    (`/Game/MainContent/Blueprints/Player/Components/Inventory/BPC_Inventory.Test_EquipItemFromFastSlot` (`self.Backpack`) 1)))

(event `InputAction|Jump`
  (params (Key :type "Key Structure"))
  ;[1 1 1] Input
  (:`Pressed`
    (`self.Jump`)
    (set `self.bJump` true))
  (:`Released`
    (`self.StopJumping`)))

(event `InputAction|Crouch`
  (params (Key :type "Key Structure"))
  ;[1 1 1] Input
  (:`Pressed`
    (`self.Crouch`)
    (set `self.bCrouch` true))
  (:`Released`
    (`self.UnCrouch`)
    (set `self.bCrouch` false)))

(event `InputAction|DropItem`
  (params (Key :type "Key Structure"))
  ;[1 1 1] Input
  (:`Pressed`
    (`self.CanDrop?`
      (:`finish`
        (`/Game/MainContent/Blueprints/Player/Components/Inventory/BPC_Inventory.DropFromHand` (`self.Backpack`) (`self.CurrentItem`))
        (`self.UnEquipItem`)))))

(event `self.OnLanded`
  (params (Hit :type "HitResult Structure (by ref)"))
  ;[1 1 1] Input
  (`KismetSystemLibrary.PrintString` "Логика приземления(звук и смена режима передвижения \"enum\")")
  (set `self.bJump` false))

(event `InputAction|Action`
  (params (Key :type "Key Structure"))
  ;[1 1 1] Input
  (:`Pressed`
    (bind _currentitem (`self.CanUseItem?`)
      (:`true`
        (`/Game/MainContent/Blueprints/Items/ItemBase/BP_ItemBase.StartUse` _currentitem))))
  (:`Released`
    (bind _currentitem_2 (`self.CanUseItem?`)
      (:`true`
        (`/Game/MainContent/Blueprints/Items/ItemBase/BP_ItemBase.StopUse` _currentitem_2)))))

(event `InputAction|Additional action`
  (params (Key :type "Key Structure"))
  ;[1 1 1] Input
  (:`Pressed`
    (`self.CanUseItem?`))
  (:`Released`
    (`self.CanUseItem?`)))

(event `InputAction|Reload`
  (params (Key :type "Key Structure"))
  ;[1 1 1] Input
  (:`Pressed`
    (bind _currentitem (`self.CanUseItem?`)
      (:`true`
        (`self.GetWeapon`
          (:`Weapon`
            (if (and (not (`self.bReload`)) (not (`self.bUseItem`)))
              (bind _asbp_weapon_core (cast `/Game/MainContent/Blueprints/Items/ItemBase/ItemsEquip/Weapons/BP_WeaponCore` _currentitem))
              (`/Game/MainContent/Blueprints/Items/ItemBase/ItemsEquip/Weapons/BP_WeaponCore.StartReload` _asbp_weapon_core))))))))

(event `Key|Q`
  (params (Key :type "Key Structure"))
  ;[1 1 1] Test
  (:`Pressed`
    (`/Engine/EditorBlueprintResources/StandardMacros.FlipFlop`
      (:`A`
        (set `self.bSwitch` true))
      (:`B`
        (set `self.bSwitch` false)))))

(event `Key|P`
  (params (Key :type "Key Structure"))
  ;[1 1 1] Test
  ;;[1 1 1] InteractInput
  (:`Pressed`
    (`/Engine/EditorBlueprintResources/StandardMacros.FlipFlop`
      (:`A`
        (`self.StopInteract`))
      (:`B`
        (`self.StartInteract`)))))

(event `Key|Five`
  (params (Key :type "Key Structure"))
  (bind _currentitem (`self.CurrentItem`))
  ;[1 1 1] Test
  (:`Pressed`
    (`/Engine/EditorBlueprintResources/StandardMacros.IsValid` _currentitem
      (:`Is Valid`
        (`KismetSystemLibrary.PrintString` (`KismetTextLibrary.Conv_TextToString` (`|FormatText` " \nIndexFromInventory : {Index} \nItem : {Item}" _ (`KismetSystemLibrary.GetDisplayName` _currentitem))) true true (struct :`G` 0.66 :`B` 1.0 :`A` 1.0) 20.0)))))

(event `Key|Zero`
  (params (Key :type "Key Structure"))
  (bind _currentitem (`self.CurrentItem`))
  (bind (_name _description _icon _equipitemclass _maxstucksize _model _itemtype _pickupitemclass _itemtypetag) (break `/Game/MainContent/Blueprints/Player/Components/Inventory/S_Item` (`/Game/MainContent/Blueprints/Items/ItemObjectForInventory/BP_ItemObjectCore.GetItemStructure` (`/Game/MainContent/Blueprints/Items/ItemBase/BP_ItemBase.ObjectCore` _currentitem))))
  ;[1 1 1] Test
  (:`Pressed`
    (`/Engine/EditorBlueprintResources/StandardMacros.IsValid` _currentitem
      (:`Is Valid`
        (`KismetSystemLibrary.PrintString` (`KismetTextLibrary.Conv_TextToString` (`|FormatText` "Name: {Name} \nDescription:{Desc} \nIcon:{Icon} \nItemClass:{ItemClass} \nMaxStuckSize:{MaxStuck} \nModel:{Model} \nItemTypeTag:{IsStack} \nItemType:{ItemType} \nPickUpItemClass:{PickUp} \nIsWear:{IsWear}" _name _description _icon (`KismetSystemLibrary.GetClassDisplayName` _equipitemclass) _maxstucksize _model (`BlueprintGameplayTagLibrary.GetTagName` _itemtypetag) (`|GetEnumeratorNameAsString` _itemtype) (`KismetSystemLibrary.GetClassDisplayName` _pickupitemclass) (`KismetSystemLibrary.IsValidClass` _pickupitemclass))) true true (struct :`R` 0.266062 :`G` 1.0 :`A` 1.0) 20.0)))))

(event `Key|B`
  (params (Key :type "Key Structure"))
  ;[1 1 1] Test
)

(event `Key|K`
  (params (Key :type "Key Structure"))
  ;[1 1 1] Test
)

(event `Key|L`
  (params (Key :type "Key Structure"))
  ;[1 1 1] Test
)

(event `self.ReceiveTick`
  (params (DeltaSeconds :type "Float (single-precision)"))
  (bind _backpack (`self.Backpack`))
  (bind _currentitem (`self.CurrentItem`))
  ;[1 1 1] Инфо о персонаже
  (`self.InfoWeaponAmmo`)
  (`KismetSystemLibrary.PrintString` "-----------------------------------------------------------------------" true true (struct :`G` 0.66 :`B` 1.0 :`A` 1.0) 0.0)
  (`self.InfoCharacter`)
  (`KismetSystemLibrary.PrintString` "-----------------------------------------------------------------------" true true (struct :`G` 0.66 :`B` 1.0 :`A` 1.0) 0.0)
  (for (_array_element _array_index) (`/Game/MainContent/Blueprints/Player/Components/Inventory/BPC_Inventory.Items` _backpack)
    (`KismetSystemLibrary.PrintString` (`KismetTextLibrary.Conv_TextToString` (`|FormatText` "{Index} : {Object}" _array_index _array_element)) true true (struct :`G` 0.66 :`B` 1.0 :`A` 1.0) 0.0))
  (`KismetSystemLibrary.PrintString` "Items" true true (struct :`G` 0.66 :`B` 1.0 :`A` 1.0) 0.0)
  (for (_array_element_2 _array_index_2) (`/Game/MainContent/Blueprints/Player/Components/Inventory/BPC_Inventory.Weapons` _backpack)
    (`KismetSystemLibrary.PrintString` (`KismetTextLibrary.Conv_TextToString` (`|FormatText` "{Index} : {Object}" _array_index_2 _array_element_2)) true true (struct :`G` 0.66 :`B` 1.0 :`A` 1.0) 0.0))
  (`KismetSystemLibrary.PrintString` "Weapons" true true (struct :`G` 0.66 :`B` 1.0 :`A` 1.0) 0.0)
  (`/Engine/EditorBlueprintResources/StandardMacros.IsValid` _currentitem
    (:`Is Valid`
      (`KismetSystemLibrary.PrintString` "-----------------------------------------------------------------------" true true (struct :`G` 0.66 :`B` 1.0 :`A` 1.0) 0.0)
      (`KismetSystemLibrary.PrintString` (`KismetTextLibrary.Conv_TextToString` (`|FormatText` "Quantity : {Quan}" (`/Game/MainContent/Blueprints/Items/ItemObjectForInventory/BP_ItemObjectCore.Quantity` (`/Game/MainContent/Blueprints/Items/ItemBase/BP_ItemBase.ObjectCore` _currentitem)))) true true (struct :`G` 0.66 :`B` 1.0 :`A` 1.0) 0.0))))

(fn `Calculate Character Speed`
  (returns (Speed :type "Float (double-precision)"))
  (return (`KismetMathLibrary.VSize` (`self.GetVelocity`))))

(fn `GetCurrentItem`
  (returns (ItemInHand :type "/Game/MainContent/Blueprints/Items/ItemBase/BP_ItemBase Object Reference"))
  (return (`self.CurrentItem`)))

(fn `GetItemObject`
  (returns (ObjectCore :type "/Game/MainContent/Blueprints/Items/ItemObjectForInventory/BP_ItemObjectCore Object Reference"))
  (return (`/Game/MainContent/Blueprints/Items/ItemBase/BP_ItemBase.ObjectCore` (`self.CurrentItem`))))

(fn `InfoCharacter`
  (`KismetSystemLibrary.PrintString` (`KismetTextLibrary.Conv_TextToString` (`|FormatText` "Speed : {Speed} \nJump : {Jump} \nCrouch : {Crouch} \nAim : {Aim} \nControlRotation : {ControlRotation} \nReload : {Reload} \nUseItem : {UseItem} \nSprint : {Sprint} \nSwitch : {Switch} \nInteract : {Interact} \nItemInHand : {ItemInHand}" (`KismetMathLibrary.VSize` (`self.GetVelocity`)) (`self.bJump`) (`NavMovementComponent.IsCrouching` (`self.CharacterMovement`)) _ (`KismetStringLibrary.Conv_RotatorToString` (`self.GetControlRotation`)) (`self.bReload`) (`self.bUseItem`) (`self.bSprint`) (`self.bSwitch`) (`self.bInteract`) (`|GetEnumeratorNameAsString` (`self.ItemInHand`)))) true true (struct :`G` 0.66 :`B` 1.0 :`A` 1.0) 0.0))

(fn `InfoWeaponAmmo`
  (bind _currentitem (`self.CurrentItem`))
  (`self.GetWeapon`
    (:`Weapon`
      (`/Engine/EditorBlueprintResources/StandardMacros.IsValid` _currentitem
        (:`Is Valid`
          (bind _asbp_weapon_core (cast `/Game/MainContent/Blueprints/Items/ItemBase/ItemsEquip/Weapons/BP_WeaponCore` _currentitem))
          (`KismetSystemLibrary.PrintString` (`KismetTextLibrary.Conv_TextToString` (`|FormatText` "CurrentAmmo : {ca} \nAllAmmo : {aa}" (`/Game/MainContent/Blueprints/Items/ItemObjectForInventory/ChildObjects/Weapon/BP_WeaponObject.CurrentAmmo` (`/Game/MainContent/Blueprints/Items/ItemBase/ItemsEquip/Weapons/BP_WeaponCore.WeaponObject` _asbp_weapon_core)) (`/Game/MainContent/Blueprints/Items/ItemBase/ItemsEquip/Weapons/BP_WeaponCore.GetCurrentMaxAmmo` _asbp_weapon_core))) true true (struct :`G` 0.66 :`B` 1.0 :`A` 1.0) 0.0))))))

(fn `IsInteractable?(????)`
  (bind (_x _y) (`KismetMathLibrary.BreakVector2D` (`WidgetLayoutLibrary.GetViewportSize`)))
  (bind (_worldposition _worlddirection) (`GameplayStatics.DeprojectScreenToWorld` (`GameplayStatics.GetPlayerController` 0) (`KismetMathLibrary.MakeVector2D` (/ _x 2.0) (/ _y 2.0))))
  (`KismetSystemLibrary.SphereTraceSingle` :`Start` _worldposition :`End` (+ _worldposition (* _worlddirection 250.0)) :`Radius` 10.0 :`TraceChannel` "TraceTypeQuery1" :`DrawDebugType` "ForDuration"))

(fn `MoveForward`
  (params (AxisForward :type "Float (double-precision)") (CanMoveFB :type Boolean))
  (if CanMoveFB
    (`self.AddMovementInput` (`KismetMathLibrary.GetForwardVector` (`KismetMathLibrary.MakeRotator` 0.0 0.0 (.yaw (`self.GetControlRotation`)))) AxisForward)))

(fn `MoveRight`
  (params (AxisRight :type "Float (double-precision)") (CanMoveLR :type Boolean))
  (if CanMoveLR
    (`self.AddMovementInput` (`KismetMathLibrary.GetRightVector` (`KismetMathLibrary.MakeRotator` 0.0 0.0 (.yaw (`self.GetControlRotation`)))) AxisRight)))

(fn `PlayPlayerAnimMontage`
  (params (CharacterMontageToPlay :type "AnimMontage Object Reference"))
  (`AnimInstance.Montage_Play` (`SkeletalMeshComponent.GetAnimInstance` (`self.Mesh`)) CharacterMontageToPlay 1.0 "MontageLength" 0.0 true))

(fn `UserConstructionScript`
  (`parent.UserConstructionScript`))