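; Player stamina component that gates sprinting and jumping by switching the owner's walk and crouch speed limits.
; StartRun enables Tick until grounded movement is detected, then a looping timer drains stamina by speed and stance, sparing falls.
; TryJump spends a fixed cost.
; Delayed timers start regeneration, faster when standing still, while a NeedRest flag blocks exhausted running and jumping until a threshold is regained.
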(event `self.ReceiveBeginPlay`
  (bind _returnvalue (`self.GetOwner`))
  (bind _output_get (set `self.OwnerCharacterMovementComponent` (`Actor.GetComponentByClass` _returnvalue "/Script/Engine.CharacterMovementComponent")))
  (`self.Save Walk Speed` _output_get)
  (set `self.CurrentStamina` (`KismetMathLibrary.Min` (`self.MaxStamina`) (`self.CurrentStamina`)))
  (set `self.OwnerHealthComponent` (`Actor.GetComponentByClass` _returnvalue "/Game/MainContent/Blueprints/Player/Components/CharacterAbilities/BPC_Health.BPC_Health_C"))
  (`self.TimerToBeginRefreshStamina`))

(event `ShowInfo`
  ;[1 1 1] TES
  (`KismetSystemLibrary.PrintString` (`KismetTextLibrary.Conv_TextToString` (`|FormatText` "RunTimer : {RT} \nRefreshStamina : {RS} \nStamina : {S}" (`KismetSystemLibrary.K2_IsTimerActive` null "RunTimerLogic") (`KismetSystemLibrary.K2_IsTimerActiveHandle` (`self.RefreshStaminaTimer`)) (`self.CurrentStamina`))) true true (struct :`G` 0.66 :`B` 1.0 :`A` 1.0) 0.0))

(event `self.ReceiveTick`
  (params (DeltaSeconds :type "Float (single-precision)"))
  (if (and (> (`self.GetOwnerSpeed`) 50.0) (not (`NavMovementComponent.IsFalling` (`self.OwnerCharacterMovementComponent`))))
    (`self.SetComponentTickEnabled` false)
    (if (not (`self.bNeedRest?`))
      (`self.SetOwnerSpeed` (`self.Run Speed`) (`self.Run Speed Crouched`))
      (`self.StopRefreshStaminaTimer`))
    (`KismetSystemLibrary.K2_SetTimer` null "RunTimerLogic" 0.25 true)))

(fn `GetOwnerSpeed`
  (returns (ReturnValue :type "Float (double-precision)"))
  (return (`KismetMathLibrary.VSize` (`Actor.GetVelocity` (`self.GetOwner`)))))

(fn `GetStamina`
  (returns (Stamina :type Integer))
  (return (`self.CurrentStamina`)))

(fn `RefreshStamina`
  (bind _returnvalue (`KismetSystemLibrary.K2_SetTimerDelegate` (`|CreateDelegate` :!event `RefreshStaminaTimerLogic`) 0.25 true))
  (set `self.RefreshStaminaTimer` _returnvalue))

(fn `RefreshStaminaTimerLogic`
  (if (== (`self.CurrentStamina`) (`self.MaxStamina`))
    (`KismetSystemLibrary.K2_ClearAndInvalidateTimerHandle` (`self.RefreshStaminaTimer`))
    (else
      (set `self.CurrentStamina` (`KismetMathLibrary.Min` (+ (`KismetMathLibrary.SelectInt` 3 2 (< (`self.GetOwnerSpeed`) 50.0)) (`self.CurrentStamina`)) (`self.MaxStamina`)))
      (`self.SetNeedRest`))))

(fn `RunTimerLogic`
  (if (or (== (`self.CurrentStamina`) 0) (`self.bNeedRest?`))
    (`self.TimerToBeginRefreshStamina`)
    (`self.SetOwnerSpeed` (`self.Start Max Walk Speed`) (`self.Start Max Walk Speed Crouched`))
    (else
      (`self.SetOwnerSpeed` (`self.Run Speed`) (`self.Run Speed Crouched`))
      (if (< (`self.GetOwnerSpeed`) 50.0)
        (`self.TimerToBeginRefreshStamina`)
        (else
          (`self.StopRefreshStaminaTimer`)
          (bind _output_get (set `self.CurrentStamina` (`KismetMathLibrary.Max` (- (`self.CurrentStamina`) (`KismetMathLibrary.SelectInt` 0 (`KismetMathLibrary.SelectInt` (`KismetMathLibrary.SelectInt` 0 2 (< (`self.GetOwnerSpeed`) (`self.Start Max Walk Speed Crouched`))) (`KismetMathLibrary.SelectInt` 0 3 (< (`self.GetOwnerSpeed`) (`self.Start Max Walk Speed`))) (`NavMovementComponent.IsCrouching` (`self.OwnerCharacterMovementComponent`))) (`NavMovementComponent.IsFalling` (`self.OwnerCharacterMovementComponent`)))))))
          (if (== _output_get 0)
            (set `self.bNeedRest?` true)
            (`self.TimerToBeginRefreshStamina`)
            (`self.SetOwnerSpeed` (`self.Start Max Walk Speed`) (`self.Start Max Walk Speed Crouched`))))))))

(fn `Save Walk Speed`
  (params (CharacterMovement :type "CharacterMovementComponent Object Reference"))
  (set `self.Start Max Walk Speed` (`CharacterMovementComponent.MaxWalkSpeed` CharacterMovement))
  (set `self.Start Max Walk Speed Crouched` (`CharacterMovementComponent.MaxWalkSpeedCrouched` CharacterMovement)))

(fn `SetNeedRest`
  (set `self.bNeedRest?` (not (>= (`self.CurrentStamina`) (`self.StaminaToFinishRest`)))))

(fn `SetOwnerSpeed`
  (params (MaxWalkSpeed :type "Float (single-precision)") (MaxWalkSpeedCrouched :type "Float (single-precision)"))
  (bind _ownercharactermovementcomponent (`self.OwnerCharacterMovementComponent`))
  (set `CharacterMovementComponent.MaxWalkSpeed` MaxWalkSpeed _ownercharactermovementcomponent)
  (set `CharacterMovementComponent.MaxWalkSpeedCrouched` MaxWalkSpeedCrouched _ownercharactermovementcomponent))

(fn `StartRun`
  (`self.SetComponentTickEnabled` true))

(fn `StopRefreshStaminaTimer`
  (bind _refreshstaminatimer (`self.RefreshStaminaTimer`))
  (if (`KismetSystemLibrary.K2_IsTimerActiveHandle` _refreshstaminatimer)
    (`KismetSystemLibrary.K2_ClearAndInvalidateTimerHandle` _refreshstaminatimer)))

(fn `StopRun`
  (`KismetSystemLibrary.K2_ClearTimer` null "RunTimerLogic")
  (`self.SetComponentTickEnabled` false)
  (`self.SetOwnerSpeed` (`self.Start Max Walk Speed`) (`self.Start Max Walk Speed Crouched`))
  (`self.SetNeedRest`)
  (`self.TimerToBeginRefreshStamina`))

(fn `TimerToBeginRefreshStamina`
  (if (and (< (`self.CurrentStamina`) (`self.MaxStamina`)) (not (`KismetSystemLibrary.K2_IsTimerActiveHandle` (`self.RefreshStaminaTimer`))))
    (bind _returnvalue (`KismetSystemLibrary.K2_SetTimerDelegate` (`|CreateDelegate` :!event `RefreshStamina`) 3.0))
    (set `self.RefreshStaminaTimer` _returnvalue)))

(fn `TryJump`
  (params (OwnerCharacter :type "Character Object Reference"))
  (if (and (>= (`self.CurrentStamina`) (`self.NeedStaminaForJump`)) (not (`NavMovementComponent.IsFalling` (`self.OwnerCharacterMovementComponent`))) (`Character.CanJump` (`local.OwnerCharacter`)) (not (`self.bNeedRest?`)))
    (`self.StopRefreshStaminaTimer`)
    (set `self.CurrentStamina` (- (`self.CurrentStamina`) (`self.NeedStaminaForJump`)))
    (`Character.Jump` (`local.OwnerCharacter`))
    (`self.SetNeedRest`)
    (`self.TimerToBeginRefreshStamina`)))