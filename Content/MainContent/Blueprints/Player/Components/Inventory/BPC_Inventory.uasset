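; Player inventory component that stores items in fixed-size Items, Weapons and FastSlots arrays and handles pickup, stacking, equipping, dropping and interaction.
; Item gameplay tags route additions to Weapons or Items, with stackable overflow spilling into further slots.
; Equipping spawns an actor on a per-type mesh socket; hotkey and mouse-wheel switching cycle Weapons plus FastSlots, remembering the last index.
; Screen-center sphere traces drive interface-based interaction and drop placement, and a toggle opens the inventory widget.
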(event `self.ReceiveBeginPlay`
  (`self.ResizeInventory`))

(fn `Add Weapon`
  (params (ItemObject :type "/Game/MainContent/Blueprints/Items/ItemObjectForInventory/BP_ItemObjectCore Object Reference"))
  (returns (Success :type Boolean))
  (bind _isadd_ (`self.CreateItemStack` (`self.Weapons`) ItemObject))
  (return _isadd_))

(fn `AddItem`
  (params (ItemObject :type "/Game/MainContent/Blueprints/Items/ItemObjectForInventory/BP_ItemObjectCore Object Reference"))
  (returns (Success :type Boolean))
  (if (`self.Is Stackable?` (`/Game/MainContent/Blueprints/Items/ItemObjectForInventory/BP_ItemObjectCore.GetItemStructure` ItemObject))
    (bind _itemtoaddstack (`self.Find Item to Stack` (`/Game/MainContent/Blueprints/Items/ItemObjectForInventory/BP_ItemObjectCore.GetItemID` (`local.ItemObject`))))
    (`/Engine/EditorBlueprintResources/StandardMacros.IsValid` _itemtoaddstack
      (:`Is Valid`
        (bind _isadd_ (`self.AddToStack` (`local.ItemObject`) _itemtoaddstack))
        (return _isadd_))
      (:`Is Not Valid`
        _)))
  (bind _isadd__2 (`self.CreateItemStack` (`self.Items`) (`local.ItemObject`)))
  (return _isadd__2))

(fn `AddToStack`
  (params (ItemObject :type "/Game/MainContent/Blueprints/Items/ItemObjectForInventory/BP_ItemObjectCore Object Reference") (ItemToAddStack :type "/Game/MainContent/Blueprints/Items/ItemObjectForInventory/BP_ItemObjectCore Object Reference"))
  (returns (`IsAdd?` :type Boolean))
  (locals (StackSize :type Integer))
  (bind ((`MaxStuckSize_10_1AD33E5548CCE857DFD4ACA09E8B119C` _maxstucksize)) (break `/Game/MainContent/Blueprints/Player/Components/Inventory/S_Item` (`/Game/MainContent/Blueprints/Items/ItemObjectForInventory/BP_ItemObjectCore.GetItemStructure` (`local.ItemToAddStack`))))
  (set `local.StackSize` (+ (`/Game/MainContent/Blueprints/Items/ItemObjectForInventory/BP_ItemObjectCore.Quantity` ItemToAddStack) (`/Game/MainContent/Blueprints/Items/ItemObjectForInventory/BP_ItemObjectCore.Quantity` ItemObject)))
  (if (<= (`local.StackSize`) (`.MaxStuckSize_10_1AD33E5548CCE857DFD4ACA09E8B119C` (break `/Game/MainContent/Blueprints/Player/Components/Inventory/S_Item` (`/Game/MainContent/Blueprints/Items/ItemObjectForInventory/BP_ItemObjectCore.GetItemStructure` ItemToAddStack))))
    (set `/Game/MainContent/Blueprints/Items/ItemObjectForInventory/BP_ItemObjectCore.Quantity` (`local.StackSize`) (`local.ItemToAddStack`))
    (set `/Game/MainContent/Blueprints/Items/ItemObjectForInventory/BP_ItemObjectCore.Quantity` 0 (`local.ItemObject`))
    (return true)
    (else
      (set `/Game/MainContent/Blueprints/Items/ItemObjectForInventory/BP_ItemObjectCore.Quantity` (- (`local.StackSize`) _maxstucksize) (`local.ItemObject`))
      (set `/Game/MainContent/Blueprints/Items/ItemObjectForInventory/BP_ItemObjectCore.Quantity` _maxstucksize (`local.ItemToAddStack`))
      (bind _success (`self.AddItem` (`local.ItemObject`)))
      (return _success))))

(fn `CanAddItem?`
  (params (Object :type "/Game/MainContent/Blueprints/Items/ItemObjectForInventory/BP_ItemObjectCore Object Reference"))
  (returns (Success :type Boolean))
  (`self.ItemType` (`.ItemTypeTag_49_7E5FAAAD4F9446B698DC2993228AB690` (break `/Game/MainContent/Blueprints/Player/Components/Inventory/S_Item` (`/Game/MainContent/Blueprints/Items/ItemObjectForInventory/BP_ItemObjectCore.GetItemStructure` Object)))
    (:`Item`
      (bind _success (`self.AddItem` Object))
      (return _success))
    (:`Weapon`
      (bind _success_2 (`self.Add Weapon` Object))
      (return _success_2))))

(fn `CreateItemStack`
  (params (TargetArray :type "Array of /Game/MainContent/Blueprints/Items/ItemObjectForInventory/BP_ItemObjectCore Object Reference") (object :type "/Game/MainContent/Blueprints/Items/ItemObjectForInventory/BP_ItemObjectCore Object Reference"))
  (returns (`IsAdd?` :type Boolean))
  (bind (_isfind_ _slotindex) (`/Game/MainContent/Blueprints/ServiceLibrary/ServiceFunctions.FindItemWithBool` TargetArray))
  (if _isfind_
    (`KismetArrayLibrary.Array_Set` TargetArray _slotindex object))
  (return _isfind_))

(fn `DropFromHand`
  (locals (ItemObject :type "/Game/MainContent/Blueprints/Items/ItemObjectForInventory/BP_ItemObjectCore Object Reference"))
  (bind _iteminhand (`self.GetPlayerCurrentItem`))
  (`/Engine/EditorBlueprintResources/StandardMacros.IsValid` _iteminhand
    (:`Is Valid`
      (bind _output_get (set `local.ItemObject` (`/Game/MainContent/Blueprints/Items/ItemBase/BP_ItemBase.GetObject` _iteminhand)))
      (bind _array (`self.GetItemArrayMacro` _output_get)
        (:`finish`
          (`self.UnEquipAndSaveIndex`)
          (`self.DropItemLogic` (`local.ItemObject`) _array))))))

(fn `DropItemLogic`
  (params (DropItem :type "/Game/MainContent/Blueprints/Items/ItemObjectForInventory/BP_ItemObjectCore Object Reference") (TargetArray :type "Array of /Game/MainContent/Blueprints/Items/ItemObjectForInventory/BP_ItemObjectCore Object Reference"))
  (bind _outhit (`self.TraceInventory` 75.0 5.0))
  (`self.MakeEmptySlot` (`local.TargetArray`) DropItem)
  (`self.SpawnDropItem` (`self.GetDropLocation` _outhit) (`local.DropItem`)))

(fn `Equip Operation`
  (params (ItemToEquip :type "/Game/MainContent/Blueprints/Items/ItemObjectForInventory/BP_ItemObjectCore Object Reference"))
  (returns (bSuccess :type Boolean))
  (`/Engine/EditorBlueprintResources/StandardMacros.IsValid` ItemToEquip
    (:`Is Valid`
      (if (`self.IsEquip?` (`/Game/MainContent/Blueprints/Items/ItemObjectForInventory/BP_ItemObjectCore.GetItemStructure` (`local.ItemToEquip`)))
        (bind _success (`self.TryEquipItem` (`local.ItemToEquip`)))
        (return _success)
        (else
          _)))
    (:`Is Not Valid`
      _))
  (return false))

(fn `EquipFromHand`
  (params (ItemSlot :type Integer))
  (locals (ItemFromInventory :type "/Game/MainContent/Blueprints/Items/ItemObjectForInventory/BP_ItemObjectCore Object Reference"))
  (bind _equipmentarray (`self.GetEquipmentArray`))
  (`self.Equip Operation` (`|GetArrayItem` _equipmentarray (`/Game/MainContent/Blueprints/ServiceLibrary/ServiceFunctions.GetClampedIndexFromArray` ItemSlot _equipmentarray))))

(fn `EquipSpawnItemLogic`
  (params (ItemObject :type "/Game/MainContent/Blueprints/Items/ItemObjectForInventory/BP_ItemObjectCore Object Reference"))
  (bind _player (`self.Player`))
  (bind _player_2 (`self.Player`))
  (bind _player_3 (`self.Player`))
  (bind ((`EquipItemClass_51_E3D0B3EC41DC869E4E07A5B343C5A2E3` _equipitemclass) (`ItemType_23_3939123540436897D2B7FB99C9705EA9` _itemtype)) (break `/Game/MainContent/Blueprints/Player/Components/Inventory/S_Item` (`/Game/MainContent/Blueprints/Items/ItemObjectForInventory/BP_ItemObjectCore.GetItemStructure` ItemObject)))
  (bind _returnvalue (`|SpawnActorFromClass` _equipitemclass (`KismetMathLibrary.MakeTransform` (0.0 0.0 0.0)) "Undefined" "OverrideRootScale" _player _player ItemObject _player))
  (`/Game/MainContent/Blueprints/Player/PlayerCore/BP_Player.SetCurrentItem` _player_2 _returnvalue)
  (`/Game/MainContent/Blueprints/Player/PlayerCore/BP_Player.SetItemInHand` _player_2 _itemtype)
  (`Actor.K2_AttachToComponent` _returnvalue (`Character.Mesh` _player_3) (`BlueprintMapLibrary.Map_Find` (`/Game/MainContent/Blueprints/Player/PlayerCore/BP_Player.GetItemSocketType` _player_3) _itemtype) "SnapToTarget" "SnapToTarget" "SnapToTarget" true))

(fn `Find Item to Stack`
  (params (AddObjectItemID :type "DataTableRowHandle Structure"))
  (returns (ItemToAddStack :type "/Game/MainContent/Blueprints/Items/ItemObjectForInventory/BP_ItemObjectCore Object Reference"))
  (locals (SlotIndex :type Integer :default -1) (ItemToAddObject :type "/Game/MainContent/Blueprints/Items/ItemObjectForInventory/BP_ItemObjectCore Object Reference"))
  (for _array_element (`self.Items`)
    (`/Engine/EditorBlueprintResources/StandardMacros.IsValid` _array_element
      (:`Is Valid`
        (if (and (`/Game/MainContent/Blueprints/ServiceLibrary/ServiceFunctions.EqualDataTableRowHandle` (`/Game/MainContent/Blueprints/Items/ItemObjectForInventory/BP_ItemObjectCore.GetItemID` _array_element) (`local.AddObjectItemID`)) (< (`/Game/MainContent/Blueprints/Items/ItemObjectForInventory/BP_ItemObjectCore.Quantity` _array_element) (`.MaxStuckSize_10_1AD33E5548CCE857DFD4ACA09E8B119C` (break `/Game/MainContent/Blueprints/Player/Components/Inventory/S_Item` (`/Game/MainContent/Blueprints/Items/ItemObjectForInventory/BP_ItemObjectCore.GetItemStructure` _array_element)))))
          (set `local.ItemToAddObject` _array_element)
          (break)))))
  (return (`local.ItemToAddObject`)))

(fn `FindItemByID`
  (params (FindItemID :type "DataTableRowHandle Structure"))
  (returns (Success :type Boolean))
  (locals (FindedObject :type "/Game/MainContent/Blueprints/Items/ItemObjectForInventory/BP_ItemObjectCore Object Reference") (IsHasItem :type Boolean))
  (for _array_element (`self.Items`)
    (`/Engine/EditorBlueprintResources/StandardMacros.IsValid` _array_element
      (:`Is Valid`
        (if (`/Game/MainContent/Blueprints/ServiceLibrary/ServiceFunctions.EqualDataTableRowHandle` (`/Game/MainContent/Blueprints/Items/ItemObjectForInventory/BP_ItemObjectCore.GetItemID` _array_element) (`local.FindItemID`))
          (set `local.IsHasItem` true)
          (break)))))
  (return (`local.IsHasItem`)))

(fn `Get Category by Tag`
  (params (GameplayTag :type "GameplayTag Structure"))
  (returns (TagCategory :type "GameplayTag Structure"))
  (if (`BlueprintGameplayTagLibrary.MatchesTag` GameplayTag (struct :`TagName` "Items"))
    (return (struct :`TagName` "Items"))
    (elif (`BlueprintGameplayTagLibrary.MatchesTag` GameplayTag (struct :`TagName` "Weapon"))
      (return (struct :`TagName` "Weapon")))))

(fn `GetDropLocation`
  (params (OutHit :type "HitResult Structure"))
  (returns (DropLocation :type "Vector Structure"))
  (bind (_bblockinghit _binitialoverlap _time _distance _location _impactpoint _normal _impactnormal _physmat _hitactor _hitcomponent _hitbonename _bonename _hititem _elementindex _faceindex _tracestart _traceend) (`GameplayStatics.BreakHitResult` OutHit))
  (return (`KismetMathLibrary.SelectVector` _impactpoint _traceend _bblockinghit)))

(fn `GetEquipmentArray`
  (returns (EquipmentArray :type "Array of /Game/MainContent/Blueprints/Items/ItemObjectForInventory/BP_ItemObjectCore Object Reference"))
  (locals (ItemSwitchArray :type "Array of /Game/MainContent/Blueprints/Items/ItemObjectForInventory/BP_ItemObjectCore Object Reference"))
  (`KismetArrayLibrary.Array_Append` (`local.ItemSwitchArray`) (`self.Weapons`))
  (`KismetArrayLibrary.Array_Append` (`local.ItemSwitchArray`) (`self.FastSlots`))
  (return (`local.ItemSwitchArray`)))

(fn `GetPlayerCurrentItem`
  (returns (ItemInHand :type "/Game/MainContent/Blueprints/Items/ItemBase/BP_ItemBase Object Reference"))
  (return (`/Game/MainContent/Blueprints/Player/PlayerCore/BP_Player.GetCurrentItem` (`self.Player`))))

(fn `Initialize Owner`
  (params (Player :type "/Game/MainContent/Blueprints/Player/PlayerCore/BP_Player Object Reference"))
  (set `self.Player` Player))

(fn `Interact`
  (bind _outhit (`self.TraceInventory` 250.0 2.5))
  (`self.TryInteract` (`.HitActor` (`GameplayStatics.BreakHitResult` _outhit))))

(fn `Is CurrentItem?`
  (params (ItemObject :type "/Game/MainContent/Blueprints/Items/ItemObjectForInventory/BP_ItemObjectCore Object Reference"))
  (returns (Success :type Boolean))
  (return (== ItemObject (`/Game/MainContent/Blueprints/Items/ItemBase/BP_ItemBase.GetObject` (`self.GetPlayerCurrentItem`)))))

(fn `Is Stackable?`
  (params (ItemStructure :type "/Game/MainContent/Blueprints/Player/Components/Inventory/S_Item Structure"))
  (returns (`IsStack?` :type Boolean))
  (return (> (`.MaxStuckSize_10_1AD33E5548CCE857DFD4ACA09E8B119C` (break `/Game/MainContent/Blueprints/Player/Components/Inventory/S_Item` ItemStructure)) 1)))

(fn `IsEquip?`
  (params (ItemStructure :type "/Game/MainContent/Blueprints/Player/Components/Inventory/S_Item Structure"))
  (returns (IsEquip :type Boolean))
  (return (`KismetSystemLibrary.IsValidClass` (`.EquipItemClass_51_E3D0B3EC41DC869E4E07A5B343C5A2E3` (break `/Game/MainContent/Blueprints/Player/Components/Inventory/S_Item` ItemStructure)))))

(fn `IsItemEmpty?`
  (params (ItemObject :type "/Game/MainContent/Blueprints/Items/ItemObjectForInventory/BP_ItemObjectCore Object Reference"))
  (if (<= (`/Game/MainContent/Blueprints/Items/ItemObjectForInventory/BP_ItemObjectCore.Quantity` ItemObject) 0)
    (bind _array (`self.GetItemArrayMacro` ItemObject)
      (:`finish`
        (`self.MakeEmptySlot` _array ItemObject)
        (`self.RefreshInventory`)))))

(fn `MakeEmptySlot`
  (params (TargetArray :type "Array of /Game/MainContent/Blueprints/Items/ItemObjectForInventory/BP_ItemObjectCore Object Reference") (DropItem :type "/Game/MainContent/Blueprints/Items/ItemObjectForInventory/BP_ItemObjectCore Object Reference"))
  (`KismetArrayLibrary.Array_Set` (`local.TargetArray`) (`KismetArrayLibrary.Array_Find` (`local.TargetArray`) DropItem))
  (bind (_isfind_ _slotindex) (`/Game/MainContent/Blueprints/ServiceLibrary/ServiceFunctions.FindItemWithBool` (`self.FastSlots`) (`local.DropItem`)))
  (if _isfind_
    (`KismetArrayLibrary.Array_Set` (`self.FastSlots`) _slotindex)))

(fn `MouseWheelSwitchItem`
  (params (MouseWheelAxis :type "Float (double-precision)"))
  (locals (ItemSwitchArray :type "Array of /Game/MainContent/Blueprints/Items/ItemObjectForInventory/BP_ItemObjectCore Object Reference") (CurrentItemSlot :type Integer :default 0) (CountForLoop :type Integer :default 0) (WheelAxis :type Integer) (LocalArrayLength :type Integer :default 0))
  (bind _iteminhand (`self.GetPlayerCurrentItem`))
  (bind _equipmentarray (`self.GetEquipmentArray`))
  (set `local.ItemSwitchArray` _equipmentarray)
  (bind _result (`/Engine/EditorBlueprintResources/StandardMacros.NegateInt` (`KismetMathLibrary.FTrunc` (`KismetMathLibrary.SignOfFloat` (`local.MouseWheelAxis`))))
    (:`  `
      (set `local.WheelAxis` _result)
      (set `local.LocalArrayLength` (`KismetArrayLibrary.Array_Length` (`local.ItemSwitchArray`)))
      (`/Engine/EditorBlueprintResources/StandardMacros.IsValid` _iteminhand
        (:`Is Valid`
          (set `local.CountForLoop` (- (`local.LocalArrayLength`) 1))
          (set `local.CurrentItemSlot` (`/Game/MainContent/Blueprints/ServiceLibrary/ServiceFunctions.WrapArrayIndex` (+ (`KismetArrayLibrary.Array_Find` (`local.ItemSwitchArray`) (`/Game/MainContent/Blueprints/Items/ItemBase/BP_ItemBase.GetObject` _iteminhand)) (`local.WheelAxis`)) (`local.LocalArrayLength`))))
        (:`Is Not Valid`
          (set `local.CountForLoop` (`local.LocalArrayLength`))
          (set `local.CurrentItemSlot` (`self.LastEquipIndex`))))
      (bind _index (`/Game/MainContent/Blueprints/ServiceLibrary/ServiceMacros.ForLoopN WithBreak` (`local.CountForLoop`) :!label _label)
        (:`LoopBody`
          (bind _return_value (`/Game/MainContent/Blueprints/ServiceLibrary/ServiceFunctions.WrapArrayIndex` (+ (`local.CurrentItemSlot`) (* _index (`local.WheelAxis`))) (`local.LocalArrayLength`)))
          (`KismetSystemLibrary.PrintString` (`KismetStringLibrary.Conv_IntToString` _return_value))
          (bind _bsuccess (`self.Equip Operation` (`|GetArrayItem` (`local.ItemSwitchArray`) _return_value)))
          (if _bsuccess
            (goto _label :!via `Break`)))))))

(fn `ResizeInventory`
  (`KismetArrayLibrary.Array_Resize` (`self.Items`) (`self.ItemsQuantity`))
  (`KismetArrayLibrary.Array_Resize` (`self.FastSlots`) (`self.FastSlotQuantity`))
  (`KismetArrayLibrary.Array_Resize` (`self.Weapons`) (`self.WeaponQuantity`)))

(fn `SpawnDropItem`
  (params (DropLocation :type "Vector Structure") (DropItem :type "/Game/MainContent/Blueprints/Items/ItemObjectForInventory/BP_ItemObjectCore Object Reference"))
  (bind _player (`self.Player`))
  (bind _returnvalue (`|SpawnActorFromClass` (`.PickUpItemClass_34_2A79DFC143C42DEB117C189E06D6DF8D` (break `/Game/MainContent/Blueprints/Player/Components/Inventory/S_Item` (`/Game/MainContent/Blueprints/Items/ItemObjectForInventory/BP_ItemObjectCore.GetItemStructure` DropItem))) (`KismetMathLibrary.MakeTransform` DropLocation) "Undefined" "OverrideRootScale" null (`local.DropItem`) (`self.Player`)))
  (`PrimitiveComponent.SetAllPhysicsLinearVelocity` (`/Game/MainContent/Blueprints/Items/ItemsPickUp/PickUpItem/BP_PickUpCore.ItemPickUp` _returnvalue) (* (`KismetMathLibrary.GetForwardVector` (`Pawn.GetControlRotation` _player)) (`KismetMathLibrary.MapRangeClamped` (`/Game/MainContent/Blueprints/Player/PlayerCore/BP_Player.Calculate Character Speed` _player) 0.0 600.0 150.0 175.0)) false)
  (return))

(fn `SwitchItem`
  (params (ItemFromInventory :type "/Game/MainContent/Blueprints/Items/ItemObjectForInventory/BP_ItemObjectCore Object Reference"))
  (`/Game/MainContent/Blueprints/Items/ItemBase/BP_ItemBase.UnEquip` (`self.GetPlayerCurrentItem`))
  (`self.UnEquipAndSaveIndex`)
  (`self.EquipSpawnItemLogic` ItemFromInventory))

(fn `Test Get Array and Index`
  (params (ItemInHand :type "/Game/MainContent/Blueprints/Items/ItemBase/BP_ItemBase Object Reference"))
  (returns (ArrayName :type String) (ItemIndex :type Integer))
  (bind _objectcore (`/Game/MainContent/Blueprints/Items/ItemBase/BP_ItemBase.GetObject` ItemInHand))
  (bind _fastslots (`self.FastSlots`))
  (bind _weapons (`self.Weapons`))
  (bind _returnvalue (`KismetArrayLibrary.Array_Contains` _weapons _objectcore))
  (bind _returnvalue_2 (`KismetArrayLibrary.Array_Contains` _fastslots _objectcore))
  (`/Engine/EditorBlueprintResources/StandardMacros.IsValid` ItemInHand
    (:`Is Valid`
      (return (`KismetMathLibrary.SelectString` "Weapons" (`KismetMathLibrary.SelectString` "FastSlot" "" _returnvalue_2) _returnvalue) (`KismetMathLibrary.SelectInt` (`KismetArrayLibrary.Array_Find` _weapons _objectcore) (`KismetMathLibrary.SelectInt` (`KismetArrayLibrary.Array_Find` _fastslots _objectcore) -1 _returnvalue_2) _returnvalue)))))

(fn `TEST_GetLastEquipIndex`
  (returns (LastEquipIndex :type Integer))
  (return (`self.LastEquipIndex`)))

(fn `ToggleInventory`
  (params (Key :type "Key Structure" :default "None"))
  (bind _returnvalue (`GameplayStatics.GetPlayerController` 0))
  (bind _returnvalue_2 (`GameplayStatics.GetPlayerController` 0))
  (`self.InventoryHUD`
    (:`then`
      (`Widget.RemoveFromParent` (`self.InventoryHUD`))
      (set `self.InventoryHUD` null)
      (`WidgetBlueprintLibrary.SetInputMode_GameOnly` _returnvalue)
      (set `PlayerController.bShowMouseCursor` false _returnvalue))
    (:`else`
      (bind _returnvalue_3 (`|CreateWidget` "/Game/MainContent/Blueprints/Player/Components/Inventory/Widget/W_InventoryMain.W_InventoryMain_C" _returnvalue_2 Key (`self.Player`)))
      (bind _output_get (set `self.InventoryHUD` _returnvalue_3))
      (`UserWidget.AddToViewport` _output_get 0)
      (`WidgetBlueprintLibrary.SetInputMode_UIOnlyEx` _returnvalue_2 _output_get)
      (set `PlayerController.bShowMouseCursor` true _returnvalue_2))))

(fn `TraceInventory`
  (params (TraceLength :type "Float (double-precision)" :default 0.0) (Radius :type "Float (double-precision)"))
  (returns (OutHit :type "HitResult Structure"))
  (bind (_x _y) (`KismetMathLibrary.BreakVector2D` (`WidgetLayoutLibrary.GetViewportSize`)))
  (bind (_worldposition _worlddirection) (`GameplayStatics.DeprojectScreenToWorld` (`GameplayStatics.GetPlayerController` 0) (`KismetMathLibrary.MakeVector2D` (/ _x 2.0) (/ _y 2.0))))
  (bind _outhit (`KismetSystemLibrary.SphereTraceSingle` :`Start` _worldposition :`End` (+ _worldposition (* _worlddirection TraceLength)) :`Radius` Radius :`TraceChannel` "TraceTypeQuery1" :`DrawDebugType` "ForDuration" :`TraceColor` (struct :`R` 0.033181 :`B` 1.0 :`A` 1.0) :`TraceHitColor` (struct :`R` 1.0 :`B` 0.684992 :`A` 1.0) :`DrawTime` 15.0))
  (return _outhit))

(fn `TryEquipItem`
  (params (ItemFromInventory :type "/Game/MainContent/Blueprints/Items/ItemObjectForInventory/BP_ItemObjectCore Object Reference"))
  (returns (Success :type Boolean))
  (`/Engine/EditorBlueprintResources/StandardMacros.IsValid` (`self.GetPlayerCurrentItem`)
    (:`Is Valid`
      (if (`self.Is CurrentItem?` (`local.ItemFromInventory`))
        (`KismetSystemLibrary.PrintString` "NoSwitch")
        (return false)
        (else
          (`self.SwitchItem` (`local.ItemFromInventory`))
          (`KismetSystemLibrary.PrintString` "Switch")
          (return true))))
    (:`Is Not Valid`
      (`self.EquipSpawnItemLogic` (`local.ItemFromInventory`))
      (`KismetSystemLibrary.PrintString` "Equip")
      (return true))))

(fn `TryInteract`
  (params (InteractActor :type "Actor Object Reference"))
  (if (`KismetSystemLibrary.DoesImplementInterface` InteractActor "/Game/MainContent/Blueprints/Items/Interfaces/BPI_Interact.BPI_Interact_C")
    (message `/Game/MainContent/Blueprints/Items/Interfaces/BPI_Interact.StartInteract` InteractActor (`self.Player`))))

(fn `TrySaveLastEquipIndex`
  (bind _equipmentarray (`self.GetEquipmentArray`))
  (bind (_isfind_ _slotindex) (`/Game/MainContent/Blueprints/ServiceLibrary/ServiceFunctions.FindItemWithBool` _equipmentarray (`/Game/MainContent/Blueprints/Items/ItemBase/BP_ItemBase.GetObject` (`self.GetPlayerCurrentItem`))))
  (set `self.LastEquipIndex` (`KismetMathLibrary.SelectInt` _slotindex (`self.LastEquipIndex`) _isfind_)))

(fn `Un Equip from Hand`
  (bind _iteminhand (`self.GetPlayerCurrentItem`))
  (`/Engine/EditorBlueprintResources/StandardMacros.IsValid` _iteminhand
    (:`Is Valid`
      (`/Game/MainContent/Blueprints/Items/ItemBase/BP_ItemBase.UnEquip` _iteminhand)
      (`self.UnEquipAndSaveIndex`))))

(fn `UnEquipAndSaveIndex`
  (`self.TrySaveLastEquipIndex`)
  (`self.UnEquipLogic`)
  (return))

(fn `UnEquipLogic`
  (`/Game/MainContent/Blueprints/Player/PlayerCore/BP_Player.SetItemType` (`self.Player`) "NewEnumerator6")
  (`Actor.K2_DestroyActor` (`self.GetPlayerCurrentItem`)))