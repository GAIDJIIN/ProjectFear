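; Flashlight component that switches a flashlight's light and glowing mesh on and off and drains its battery.
; It receives the mesh, light source and flashlight object through InitializeProperties, and TurnOnStart applies the object's enabled state if charge remains.
; ToggleLight sets light visibility and a material scalar for the glow.
; A looping timer calls WasteEnergy to decrement the object's battery, clearing itself and switching the light off when empty.
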(fn `InitializeProperties`
  (params (FlashlightMesh :type "StaticMeshComponent Object Reference") (FlashlightSource :type "SpotLightComponent Object Reference") (FlashlightObject :type "/Game/MainContent/Blueprints/Items/ItemObjectForInventory/ChildObjects/BP_FlashLightObject Object Reference"))
  (set `self.FlashlightMesh` FlashlightMesh)
  (set `self.FlashlightSource` FlashlightSource)
  (set `self.Flashlight Object` FlashlightObject))

(fn `SetTimerWasteTime`
  (bind _returnvalue (`KismetSystemLibrary.K2_SetTimer` null "WasteEnergy" 0.5 true))
  (set `self.WasteBatteryEnergyTimer` _returnvalue))

(fn `ToggleLight`
  (params (`On&Off` :type Boolean))
  (`SceneComponent.SetVisibility` (`self.FlashlightSource`) `On&Off` false)
  (`MeshComponent.SetScalarParameterValueOnMaterials` (`self.FlashlightMesh`) (`self.LightSourceMaterialName`) (`KismetMathLibrary.SelectFloat` 3.0 0.0 `On&Off`)))

(fn `TurnOnStart`
  (bind _flashlight_object (`self.Flashlight Object`))
  (bind _isenable_ (`/Game/MainContent/Blueprints/Items/ItemObjectForInventory/ChildObjects/BP_FlashLightObject.IsEnable?` _flashlight_object))
  (if (> (`/Game/MainContent/Blueprints/Items/ItemObjectForInventory/ChildObjects/BP_FlashLightObject.BatteryEnergy` _flashlight_object) 0)
    (`self.ToggleLight` _isenable_)
    (if _isenable_
      (`self.SetTimerWasteTime`))))

(fn `WasteEnergy`
  (if (> (`/Game/MainContent/Blueprints/Items/ItemObjectForInventory/ChildObjects/BP_FlashLightObject.BatteryEnergy` (`self.Flashlight Object`)) 0)
    (`/Engine/EditorBlueprintResources/StandardMacros.DecrementInt` (`/Game/MainContent/Blueprints/Items/ItemObjectForInventory/ChildObjects/BP_FlashLightObject.BatteryEnergy` (`self.Flashlight Object`)))
    (else
      (`KismetSystemLibrary.K2_ClearAndInvalidateTimerHandle` (`self.WasteBatteryEnergyTimer`))
      (`self.ToggleLight` false))))