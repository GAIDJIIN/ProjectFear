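; Player component that handles aim-down-sights by moving the first-person camera between the player's camera socket and a socket on the aimed actor's mesh.
; StartADS restarts the timer for the requested direction, with a short delay before moving in.
; Looping timers, rather than Tick, step an alpha through curves to blend camera location and FOV.
; Moving out clears the timer and resets FOV on arrival; GetIsADS exposes the aiming state.
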(event `self.ReceiveBeginPlay`
  (`self.InitializeInfo`))

(fn `GetIsADS`
  (returns (bADS :type Boolean))
  (return (`self.bADS`)))

(fn `InitializeInfo`
  (bind _output_get (set `self.Player` (cast `/Game/MainContent/Blueprints/Player/PlayerCore/BP_Player` (`self.GetOwner`) :!pure true)))
  (set `self.F_Camera` (`/Game/MainContent/Blueprints/Player/PlayerCore/BP_Player.F_Camera` _output_get))
  (set `self.ADSTimer` 0.0))

(fn `Move Camera Out`
  (bind _camerasocketlocation (`/Game/MainContent/Blueprints/Player/PlayerCore/BP_Player.GetCameraSocketLocation` (`self.Player`)))
  (`self.Player`
    (:`then`
      (`self.F_Camera`
        (:`then`
          (if (== (`SceneComponent.K2_GetComponentLocation` (`self.F_Camera`)) _camerasocketlocation :`ErrorTolerance` 0.01)
            (`KismetSystemLibrary.K2_ClearAndInvalidateTimerHandle` (`self.ADSTimerHandle`))
            (set `self.ADSTimer` 0.0)
            (`CameraComponent.SetFieldOfView` (`self.F_Camera`) 90.0)
            (else
              (`SceneComponent.K2_SetWorldLocation` (`self.F_Camera`) (`KismetMathLibrary.VLerp` _camerasocketlocation (`SceneComponent.K2_GetComponentLocation` (`self.F_Camera`)) (`CurveFloat.GetFloatValue` (`self.ADSCurve`) (`self.ADSTimer`))) false false)
              (`CameraComponent.SetFieldOfView` (`self.F_Camera`) (`KismetMathLibrary.Lerp` 90.0 70.0 (`CurveFloat.GetFloatValue` (`self.FOV_ADS`) (`self.ADSTimer`))))
              (set `self.ADSTimer` (`KismetMathLibrary.FMax` (- (`self.ADSTimer`) 0.045))))))
        (:`else`)))
    (:`else`)))

(fn `MoveCamera In`
  (bind _player (`self.Player`))
  (bind (_scenecomponent _sockettomove) (message `/Game/MainContent/Blueprints/Player/InterfacesForPlayer/BPI_MoveCamera.GetMeshInfo` (`self.ActorToMove`)))
  (`/Engine/EditorBlueprintResources/StandardMacros.IsValid` _player
    (:`Is Valid`
      (`/Engine/EditorBlueprintResources/StandardMacros.IsValid` (`self.F_Camera`)
        (:`Is Valid`
          (bind _returnvalue (`SceneComponent.GetSocketLocation` _scenecomponent _sockettomove))
          (if (not (== (`SceneComponent.K2_GetComponentLocation` (`self.F_Camera`)) _returnvalue :`ErrorTolerance` 0.01))
            (`SceneComponent.K2_SetWorldLocation` (`self.F_Camera`) (`KismetMathLibrary.VLerp` (`/Game/MainContent/Blueprints/Player/PlayerCore/BP_Player.GetCameraSocketLocation` _player) _returnvalue (`CurveFloat.GetFloatValue` (`self.ADSCurve`) (`self.ADSTimer`))) false false)
            (`CameraComponent.SetFieldOfView` (`self.F_Camera`) (`KismetMathLibrary.Lerp` 90.0 70.0 (`CurveFloat.GetFloatValue` (`self.FOV_ADS`) (`self.ADSTimer`))))
            (set `self.ADSTimer` (`KismetMathLibrary.FMin` (+ (`self.ADSTimer`) 0.035) 1.0))))))))

(fn `Start ADS`
  (params (MoveCameraMode :type "/Game/MainContent/Blueprints/Player/InterfacesForPlayer/E_MoveCameraMode Enum" :default "NewEnumerator0") (ActorToMove :type "Actor Object Reference"))
  (bind _adstimerhandle (`self.ADSTimerHandle`))
  (bind _output_get (set `self.ActorToMove` ActorToMove))
  (`/Engine/EditorBlueprintResources/StandardMacros.IsValid` _output_get
    (:`Is Valid`
      (if (`KismetSystemLibrary.K2_IsTimerActiveHandle` _adstimerhandle)
        (`KismetSystemLibrary.K2_ClearAndInvalidateTimerHandle` _adstimerhandle))
      (switch `/Game/MainContent/Blueprints/Player/InterfacesForPlayer/E_MoveCameraMode` MoveCameraMode
        (:`NewEnumerator0`
          (bind _returnvalue (`KismetSystemLibrary.K2_SetTimerDelegate` (`|CreateDelegate` :!event `WaitToMoveCameraIn`) 0.075))
          (set `self.ADSTimerHandle` _returnvalue))
        (:`NewEnumerator1`
          (`self.WaitToMoveCameraOut`))))))

(fn `WaitToMoveCameraIn`
  (set `self.bADS` true)
  (bind _returnvalue (`KismetSystemLibrary.K2_SetTimerDelegate` (`|CreateDelegate` :!event `MoveCamera In`) 0.0075 true))
  (set `self.ADSTimerHandle` _returnvalue))

(fn `WaitToMoveCameraOut`
  (set `self.bADS` false)
  (bind _returnvalue (`KismetSystemLibrary.K2_SetTimerDelegate` (`|CreateDelegate` :!event `Move Camera Out`) 0.0075 true))
  (set `self.ADSTimerHandle` _returnvalue))