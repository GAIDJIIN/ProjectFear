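; Player component that handles aim-down-sights by sliding the player's camera to a socket on a target actor and narrowing its FOV.
; StartADS starts looping timers for zooming in, after a short delay, or for zooming out immediately.
; Each step blends location and FOV through curves, using sockets from the player mesh and the target's GetMeshInfoMessage.
; Zoom-out clears the timer and target once the camera is back at its socket.
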(event `self.ReceiveBeginPlay`
  (`self.InitializeInfo`))

(fn `GetIsADS`
  (returns (bADS :type Boolean))
  (return (`self.bADS`)))

(fn `InitializeInfo`
  (bind _output_get (set `self.Player` (cast `/Game/MainContent/Blueprints/Player/PlayerCore/BP_Player` (`self.GetOwner`) :!pure true)))
  (set `self.F_Camera` (`Actor.GetComponentByClass` _output_get "/Script/Engine.CameraComponent"))
  (set `self.ADSTimer` 0.0))

(fn `Move Camera Out`
  (bind _returnvalue (`SceneComponent.GetSocketLocation` (`Character.Mesh` (`self.Player`)) (`SceneComponent.GetAttachSocketName` (`self.F_Camera`))))
  (`self.Player`
    (:`then`
      (`self.F_Camera`
        (:`then`
          (if (== (`SceneComponent.K2_GetComponentLocation` (`self.F_Camera`)) _returnvalue :`ErrorTolerance` 0.01)
            (`KismetSystemLibrary.K2_ClearAndInvalidateTimerHandle` (`self.ADSTimerHandle`))
            (set `self.ADSTimer` 0.0)
            (`CameraComponent.SetFieldOfView` (`self.F_Camera`) 90.0)
            (set `self.ActorToMove` null)
            (else
              (`SceneComponent.K2_SetWorldLocation` (`self.F_Camera`) (`KismetMathLibrary.VLerp` _returnvalue (`SceneComponent.K2_GetComponentLocation` (`self.F_Camera`)) (`CurveFloat.GetFloatValue` (`self.ADSCurve`) (`self.ADSTimer`))) false false)
              (`CameraComponent.SetFieldOfView` (`self.F_Camera`) (`KismetMathLibrary.Lerp` 90.0 70.0 (`CurveFloat.GetFloatValue` (`self.FOV_ADS`) (`self.ADSTimer`))))
              (set `self.ADSTimer` (`KismetMathLibrary.FMax` (- (`self.ADSTimer`) 0.045))))))
        (:`else`)))
    (:`else`)))

(fn `MoveCamera In`
  (bind _actortomove (`self.ActorToMove`)
    (:`then`
      (bind (_scenecomponent _sockettomove) (message `/Game/MainContent/Blueprints/Player/InterfacesForPlayer/BPI_MoveCamera.GetMeshInfo` _actortomove))
      (`self.Player`
        (:`then`
          (`self.F_Camera`
            (:`then`
              (bind _returnvalue (`SceneComponent.GetSocketLocation` _scenecomponent _sockettomove))
              (if (not (== (`SceneComponent.K2_GetComponentLocation` (`self.F_Camera`)) _returnvalue :`ErrorTolerance` 0.01))
                (`SceneComponent.K2_SetWorldLocation` (`self.F_Camera`) (`KismetMathLibrary.VLerp` (`SceneComponent.GetSocketLocation` (`Character.Mesh` (`self.Player`)) (`SceneComponent.GetAttachSocketName` (`self.F_Camera`))) _returnvalue (`CurveFloat.GetFloatValue` (`self.ADSCurve`) (`self.ADSTimer`))) false false)
                (`CameraComponent.SetFieldOfView` (`self.F_Camera`) (`KismetMathLibrary.Lerp` 90.0 70.0 (`CurveFloat.GetFloatValue` (`self.FOV_ADS`) (`self.ADSTimer`))))
                (set `self.ADSTimer` (`KismetMathLibrary.FMin` (+ (`self.ADSTimer`) 0.035) 1.0))))
            (:`else`)))
        (:`else`)))
    (:`else`)))

(fn `Start ADS`
  (params (MoveCameraMode :type "/Game/MainContent/Blueprints/Player/InterfacesForPlayer/E_MoveCameraMode Enum" :default "NewEnumerator0") (ActorToMove :type "Actor Object Reference"))
  (bind _adstimerhandle (`self.ADSTimerHandle`))
  (`/Engine/EditorBlueprintResources/StandardMacros.IsValid` ActorToMove
    (:`Is Valid`
      (set `self.ActorToMove` ActorToMove)
      (if (`KismetSystemLibrary.K2_IsTimerActiveHandle` _adstimerhandle)
        (`KismetSystemLibrary.K2_ClearAndInvalidateTimerHandle` _adstimerhandle))
      (switch `/Game/MainContent/Blueprints/Player/InterfacesForPlayer/E_MoveCameraMode` MoveCameraMode
        (:`NewEnumerator0`
          (bind _returnvalue (`KismetSystemLibrary.K2_SetTimerDelegate` (`|CreateDelegate` :!event `WaitToMoveCameraIn`) 0.075))
          (set `self.ADSTimerHandle` _returnvalue))
        (:`NewEnumerator1`
          (`self.WaitToMoveCameraOut`))))))

(fn `WaitToMoveCameraIn`
  (set `self.bADS` true)
  (bind _returnvalue (`KismetSystemLibrary.K2_SetTimerDelegate` (`|CreateDelegate` :!event `MoveCamera In`) 0.0075 true))
  (set `self.ADSTimerHandle` _returnvalue))

(fn `WaitToMoveCameraOut`
  (set `self.bADS` false)
  (bind _returnvalue (`KismetSystemLibrary.K2_SetTimerDelegate` (`|CreateDelegate` :!event `Move Camera Out`) 0.0075 true))
  (set `self.ADSTimerHandle` _returnvalue))