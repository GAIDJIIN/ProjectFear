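; Character component that manages stamina for sprinting and jumping, and exposes Health and Stamina getters.
; StartRun raises walk speed while a looping timer drains stamina during grounded movement, and TryJump deducts a fixed cost.
; Stopping or jumping starts a delayed, timer-driven refill that regenerates faster when nearly stationary, with one handle shared by delay and refill.
; Tick prints stamina on screen as debug output.
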(event `self.ReceiveBeginPlay`
  (set `self.OwnerCharacterMovementComponent` (`Actor.GetComponentByClass` (`self.GetOwner`) "/Script/Engine.CharacterMovementComponent")))

(event `self.ReceiveTick`
  (params (DeltaSeconds :type "Float (single-precision)"))
  (`KismetSystemLibrary.PrintString` (`KismetTextLibrary.Conv_TextToString` (`|FormatText` "Stamina : {Stamina}" (`self.Stamina`))) true true (struct :`R` 1.0 :`B` 0.008162 :`A` 1.0) 0.0))

(fn `GetHealth`
  (returns (Health :type Integer))
  (return (`self.Health`)))

(fn `GetStamina`
  (returns (Stamina :type Integer))
  (return (`self.Stamina`)))

(fn `RefreshStamina`
  (bind _returnvalue (`KismetSystemLibrary.K2_SetTimerDelegate` (`|CreateDelegate` :!event `RefreshStaminaTimerLogic`) 0.25 true))
  (set `self.RefreshStaminaTimer` _returnvalue))

(fn `RefreshStaminaTimerLogic`
  (if (== (`self.Stamina`) (`self.MaxStamina`))
    (`KismetSystemLibrary.K2_ClearAndInvalidateTimerHandle` (`self.RefreshStaminaTimer`))
    (else
      (set `self.Stamina` (`KismetMathLibrary.Clamp` (+ (`KismetMathLibrary.SelectInt` 4 2 (< (`KismetMathLibrary.VSize` (`Actor.GetVelocity` (`self.GetOwner`))) 75.0)) (`self.Stamina`)) 0 (`self.MaxStamina`))))))

(fn `RunTimerLogic`
  (bind _stamina (`self.Stamina`))
  (if (== _stamina 0)
    (`self.StopRun`)
    (else
      (set `self.Stamina` (- _stamina (`KismetMathLibrary.SelectInt` 0 1 (or (< (`KismetMathLibrary.VSize` (`Actor.GetVelocity` (`self.GetOwner`))) 75.0) (`NavMovementComponent.IsFalling` (`self.OwnerCharacterMovementComponent`)))))))))

(fn `StartRun`
  (if (and (not (`NavMovementComponent.IsFalling` (`self.OwnerCharacterMovementComponent`))) (> (`self.Stamina`) 0))
    (set `self.Start Max Walk Speed` (`CharacterMovementComponent.MaxWalkSpeed` (`self.OwnerCharacterMovementComponent`)))
    (`self.StopRefreshStaminaTimer`)
    (`KismetSystemLibrary.K2_SetTimer` null "RunTimerLogic" 0.125 true)
    (set `CharacterMovementComponent.MaxWalkSpeed` (`self.Run Speed`) (`self.OwnerCharacterMovementComponent`))))

(fn `StopRefreshStaminaTimer`
  (bind _refreshstaminatimer (`self.RefreshStaminaTimer`))
  (if (`KismetSystemLibrary.K2_IsTimerActiveHandle` _refreshstaminatimer)
    (`KismetSystemLibrary.K2_ClearAndInvalidateTimerHandle` _refreshstaminatimer)))

(fn `StopRun`
  (`KismetSystemLibrary.K2_ClearTimer` null "RunTimerLogic")
  (set `CharacterMovementComponent.MaxWalkSpeed` (`self.Start Max Walk Speed`) (`self.OwnerCharacterMovementComponent`))
  (`self.TimerToBeginRefreshStamina`))

(fn `TimerToBeginRefreshStamina`
  (bind _returnvalue (`KismetSystemLibrary.K2_SetTimerDelegate` (`|CreateDelegate` :!event `RefreshStamina`) 5.0))
  (set `self.RefreshStaminaTimer` _returnvalue))

(fn `TryJump`
  (params (OwnerCharacter :type "Character Object Reference"))
  (if (and (> (`self.Stamina`) 15) (not (`NavMovementComponent.IsFalling` (`self.OwnerCharacterMovementComponent`))) (`Character.CanJump` (`local.OwnerCharacter`)))
    (`self.StopRefreshStaminaTimer`)
    (set `self.Stamina` (- (`self.Stamina`) 15))
    (`Character.Jump` (`local.OwnerCharacter`))
    (`self.TimerToBeginRefreshStamina`)))