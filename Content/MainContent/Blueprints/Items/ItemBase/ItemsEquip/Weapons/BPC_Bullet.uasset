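; BPC_Bullet is a weapon component, going by its name and path, that provides hitscan bullet hits on physics objects.
; BulletTrace runs one Visibility line trace from the muzzle along the fire vector, ignoring the given character and drawing debug lines.
; Hit components simulating physics receive a fixed-strength impulse at the impact point along the shot direction.
; The NumberOfBullets input is unused, and no damage is applied.
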(fn `BulletTrace`
  (params (NumberOfBullets :type Integer) (`Ignore Character` :type "Actor Object Reference") (`Muzzle Location` :type "Vector Structure") (`Fire Vector` :type "Vector Structure"))
  (bind _muzzle_location (`local.Muzzle Location`))
  (bind _outhit (`KismetSystemLibrary.LineTraceSingle` _muzzle_location (+ _muzzle_location (`local.Fire Vector`)) "TraceTypeQuery1" false (`|MakeArray` `Ignore Character`) "ForDuration" true (struct :`R` 1.0 :`A` 1.0) (struct :`G` 1.0 :`A` 1.0) 10.0))
  (bind (_bblockinghit _binitialoverlap _time _distance _location _impactpoint _normal _impactnormal _physmat _hitactor _hitcomponent _hitbonename _bonename _hititem _elementindex _faceindex _tracestart) (`GameplayStatics.BreakHitResult` _outhit))
  (if _bblockinghit
    (`/Engine/EditorBlueprintResources/StandardMacros.IsValid` _hitcomponent
      (:`Is Valid`
        (if (`SceneComponent.IsSimulatingPhysics` _hitcomponent _bonename)
          (`PrimitiveComponent.AddImpulseAtLocation` _hitcomponent (* (`KismetMathLibrary.GetForwardVector` (`KismetMathLibrary.FindLookAtRotation` _tracestart _impactpoint)) 4000.0) _impactpoint _bonename))))))