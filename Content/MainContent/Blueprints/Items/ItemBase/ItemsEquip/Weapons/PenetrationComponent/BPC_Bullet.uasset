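; Weapon component that fires hitscan bullets with distance falloff and surface-based penetration.
; MakeShot starts a line trace, and each hit applies physics impulse and point damage, reduces penetration by surface type, and spawns decals and effects.
; To find exit points, it multi-traces backwards from beyond the hit actor's bounds and checks thickness against per-surface limits.
; Successful penetrations recursively trace the remaining range, with debug prints and drawing throughout.
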(fn `BulletPenetrationLogic`
  (params (Direction :type "Vector Structure") (EnterLocation :type "Vector Structure") (HitActor :type "Actor Object Reference"))
  (returns (bSuccess :type Boolean) (PenetrationLocation :type "Vector Structure"))
  (bind (_origin _boxextent) (`Actor.GetActorBounds` HitActor true true))
  (bind _returnvalue (+ (`local.EnterLocation`) (* (* (`KismetMathLibrary.FMax` (.x _boxextent) (.y _boxextent) (.z _boxextent)) 2.05) (`local.Direction`))))
  (`KismetSystemLibrary.DrawDebugSphere` _returnvalue 20.0 12 (struct :`G` 1.0 :`B` 0.022145 :`A` 1.0) 10.0)
  (`KismetSystemLibrary.DrawDebugSphere` (`local.EnterLocation`) 20.0 12 (struct :`R` 1.0 :`B` 0.019095 :`A` 1.0) 10.0)
  (bind _outhits (`KismetSystemLibrary.LineTraceMulti` :`Start` _returnvalue :`End` (`local.EnterLocation`) :`TraceChannel` "TraceTypeQuery3" :`DrawDebugType` "ForDuration" :`DrawTime` 10.0))
  (if (`KismetArrayLibrary.Array_IsEmpty` _outhits)
    (return false (0.0 0.0 0.0))
    (else
      (bind (_arrayindex _arrayelement) (`/Engine/EditorBlueprintResources/StandardMacros.ReverseForEachLoop` _outhits)
        (:`LoopBody`
          (bind (_bblockinghit _binitialoverlap _time _distance _location _impactpoint _normal _impactnormal _physmat _hitactor) (`GameplayStatics.BreakHitResult` _arrayelement))
          (if (== _hitactor (`local.HitActor`))
            (bind _returnvalue_2 (`GameplayStatics.GetSurfaceType` _arrayelement))
            (if (`self.Can Penetrate Distance` (`KismetMathLibrary.Vector_Distance` _impactpoint (`local.EnterLocation`)) _returnvalue_2)
              (bind (_value _returnvalue_3) (`BlueprintMapLibrary.Map_Find` (`self.DecalBySurface`) _returnvalue_2))
              (`self.DebugSurfaceInfo` _returnvalue_3 "Don't Add Surface Type Last Decal")
              (`self.SpawnDecal` _value _arrayelement)
              (return true (+ _impactpoint (* _impactnormal 4.0)))
              (else
                (return false (0.0 0.0 0.0))))))))))

(fn `BulletTrace`
  (params (StartLocation :type "Vector Structure") (`Fire Vector` :type "Vector Structure") (`Current Bullet Info` :type "/Game/MainContent/Blueprints/Items/ItemBase/ItemsEquip/Weapons/PenetrationComponent/S_BulletInfo Structure (by ref)"))
  (bind _returnvalue (`self.GetOwner`))
  (bind _outhit (`KismetSystemLibrary.LineTraceSingle` StartLocation (+ StartLocation (`local.Fire Vector`)) "TraceTypeQuery4" false (`|MakeArray` _returnvalue (`Actor.GetOwner` _returnvalue)) "ForDuration" true (struct :`R` 1.0 :`A` 1.0) (struct :`G` 1.0 :`A` 1.0) 10.0))
  (if (`GameplayStatics.BreakHitResult` _outhit)
    (`self.HitLogic` _outhit `Current Bullet Info`)
    (else
      (`KismetArrayLibrary.Array_RemoveItem` (`self.BulletsInfo`) `Current Bullet Info`))))

(fn `Calculate Damage`
  (params (`Bullet Info` :type "/Game/MainContent/Blueprints/Items/ItemBase/ItemsEquip/Weapons/PenetrationComponent/S_BulletInfo Structure (by ref)"))
  (returns (ReturnValue :type "Float (double-precision)"))
  (bind ((`BulletDistance_5_28C69CC740FA69B50435CBAEFF733635` _bulletdistance) (`BulletDamage_6_B46BBAFF459B99B97180719B73692C9D` _bulletdamage)) (break `/Game/MainContent/Blueprints/Items/ItemBase/ItemsEquip/Weapons/PenetrationComponent/S_BulletInfo` `Bullet Info`))
  (return (* (`KismetMathLibrary.MapRangeClamped` (`self.CalculateBulletPenetrationByDistance` `Bullet Info`) 0.0 (`self.BulletPenetration`) (`self.Ratio Penetration`) 1.0) (`KismetMathLibrary.MapRangeClamped` _bulletdistance 150.0 (`self.DamageFalloffDistance`) _bulletdamage (/ _bulletdamage 4.0)))))

(fn `CalculateBulletPenetrationByDistance`
  (params (`Bullet Info` :type "/Game/MainContent/Blueprints/Items/ItemBase/ItemsEquip/Weapons/PenetrationComponent/S_BulletInfo Structure (by ref)"))
  (returns (`Calculated Penetration` :type "Float (double-precision)"))
  (bind ((`BulletPenetration_2_78026D8949F6293A426722AEEBEF7902` _bulletpenetration) (`BulletDistance_5_28C69CC740FA69B50435CBAEFF733635` _bulletdistance)) (break `/Game/MainContent/Blueprints/Items/ItemBase/ItemsEquip/Weapons/PenetrationComponent/S_BulletInfo` `Bullet Info`))
  (return (`KismetMathLibrary.MapRangeClamped` _bulletdistance 250.0 (`self.PenetrationFalloffDistance`) _bulletpenetration)))

(fn `CalculateDistance`
  (params (Distance :type "Float (double-precision)") (CurrentBulletInfo :type "/Game/MainContent/Blueprints/Items/ItemBase/ItemsEquip/Weapons/PenetrationComponent/S_BulletInfo Structure (by ref)"))
  (setmembers `/Game/MainContent/Blueprints/Items/ItemBase/ItemsEquip/Weapons/PenetrationComponent/S_BulletInfo` :`StructRef` CurrentBulletInfo :`BulletDistance` (+ Distance (`.BulletDistance_5_28C69CC740FA69B50435CBAEFF733635` (break `/Game/MainContent/Blueprints/Items/ItemBase/ItemsEquip/Weapons/PenetrationComponent/S_BulletInfo` CurrentBulletInfo)))))

(fn `Can Penetrate Distance`
  (params (PenetrationDistance :type "Float (double-precision)") (SurfaceType :type "EPhysicalSurface Enum" :default "SurfaceType_Default"))
  (returns (bCanPenetrate :type Boolean))
  (bind (_value _returnvalue) (`BlueprintMapLibrary.Map_Find` (`self.PenetrationDistanceBySurface`) (`local.SurfaceType`)))
  (return (select `bool` (or (== _value 0.0) (not _returnvalue)) :`false` (<= (`local.PenetrationDistance`) (`KismetMathLibrary.SelectFloat` 350.0 _value (< _value 0.0))))))

(fn `DebugBulletInfo`
  (params (Distance :type "Float (double-precision)") (Penetration :type "Float (double-precision)") (Damage :type "Float (double-precision)") (PrintDuration :type "Float (single-precision)" :default 15.0))
  (`KismetSystemLibrary.PrintString` (`KismetTextLibrary.Conv_TextToString` (`|FormatText` "------------------------ \nDistance : {D} \nPenetration : {P} \nDamage : {DMG}" Distance Penetration Damage)) true true (struct :`G` 1.0 :`B` 0.009347 :`A` 1.0) PrintDuration))

(fn `DebugSurfaceInfo`
  (params (bStatus :type Boolean) (InString :type String))
  (if (not bStatus)
    (`KismetSystemLibrary.PrintString` InString true true (struct :`R` 1.0 :`B` 0.048431 :`A` 1.0) 15.0)))

(fn `GetPenetrationBySurface`
  (params (SurfaceType :type "EPhysicalSurface Enum" :default "SurfaceType_Default") (BulletInfo :type "/Game/MainContent/Blueprints/Items/ItemBase/ItemsEquip/Weapons/PenetrationComponent/S_BulletInfo Structure"))
  (returns (StopPenetrationBySurface :type "Float (double-precision)"))
  (bind (_value _returnvalue) (`BlueprintMapLibrary.Map_Find` (`self.PenetrationlBySurface`) SurfaceType))
  (return (`KismetMathLibrary.SelectFloat` (+ (`.BulletPenetration_2_78026D8949F6293A426722AEEBEF7902` (break `/Game/MainContent/Blueprints/Items/ItemBase/ItemsEquip/Weapons/PenetrationComponent/S_BulletInfo` BulletInfo)) 0.1) _value (or (< _value 0.0) (not _returnvalue)))))

(fn `GetShotDirection`
  (params (Hit :type "HitResult Structure"))
  (returns (Direction :type "Vector Structure"))
  (bind (_bblockinghit _binitialoverlap _time _distance _location _impactpoint _normal _impactnormal _physmat _hitactor _hitcomponent _hitbonename _bonename _hititem _elementindex _faceindex _tracestart _traceend) (`GameplayStatics.BreakHitResult` Hit))
  (return (`KismetMathLibrary.GetForwardVector` (`KismetMathLibrary.FindLookAtRotation` _tracestart _traceend))))

(fn `HitLogic`
  (params (Hit :type "HitResult Structure") (CurrentBulletInfo :type "/Game/MainContent/Blueprints/Items/ItemBase/ItemsEquip/Weapons/PenetrationComponent/S_BulletInfo Structure (by ref)"))
  (bind _calculated_penetration (`self.CalculateBulletPenetrationByDistance` CurrentBulletInfo))
  (bind _returnvalue (`self.GetOwner`))
  (bind _hit (`local.Hit`))
  (bind ((`BulletDistance_5_28C69CC740FA69B50435CBAEFF733635` _bulletdistance) (`BulletDamage_6_B46BBAFF459B99B97180719B73692C9D` _bulletdamage)) (break `/Game/MainContent/Blueprints/Items/ItemBase/ItemsEquip/Weapons/PenetrationComponent/S_BulletInfo` (`local.CurrentBulletInfo`)))
  (bind (_bblockinghit _binitialoverlap _time _distance _location _impactpoint _normal _impactnormal _physmat _hitactor) (`GameplayStatics.BreakHitResult` _hit))
  (bind (_value _returnvalue_2) (`BlueprintMapLibrary.Map_Find` (`self.DecalBySurface`) (`GameplayStatics.GetSurfaceType` (`local.Hit`))))
  (bind (_value_2 _returnvalue_3) (`BlueprintMapLibrary.Map_Find` (`self.LastDecalBySurface`) (`GameplayStatics.GetSurfaceType` (`local.Hit`))))
  (bind _returnvalue_4 (- (`self.Distance`) (`.BulletDistance_5_28C69CC740FA69B50435CBAEFF733635` (break `/Game/MainContent/Blueprints/Items/ItemBase/ItemsEquip/Weapons/PenetrationComponent/S_BulletInfo` (`local.CurrentBulletInfo`)))))
  (`self.MakeImpulse` Hit)
  (`self.CalculateDistance` (`.Distance` (`GameplayStatics.BreakHitResult` Hit)) CurrentBulletInfo)
  (setmembers `/Game/MainContent/Blueprints/Items/ItemBase/ItemsEquip/Weapons/PenetrationComponent/S_BulletInfo` :`StructRef` CurrentBulletInfo :`BulletDamage` (`self.Calculate Damage` CurrentBulletInfo))
  ;[1 1 1] DEBUG
  (`self.DebugBulletInfo` _bulletdistance _calculated_penetration _bulletdamage 5.0)
  (setmembers `/Game/MainContent/Blueprints/Items/ItemBase/ItemsEquip/Weapons/PenetrationComponent/S_BulletInfo` :`StructRef` CurrentBulletInfo :`BulletPenetration` (- _calculated_penetration (`self.GetPenetrationBySurface` (`GameplayStatics.GetSurfaceType` Hit) CurrentBulletInfo)))
  (`GameplayStatics.ApplyPointDamage` (`.HitActor` (`GameplayStatics.BreakHitResult` (`local.Hit`))) (`.BulletDamage_6_B46BBAFF459B99B97180719B73692C9D` (break `/Game/MainContent/Blueprints/Items/ItemBase/ItemsEquip/Weapons/PenetrationComponent/S_BulletInfo` (`local.CurrentBulletInfo`))) (`self.GetShotDirection` (`local.Hit`)) (`local.Hit`) (`Pawn.GetController` (`Actor.Instigator` _returnvalue)) _returnvalue (`self.Damage Type Class`))
  (if (>= (`.BulletPenetration_2_78026D8949F6293A426722AEEBEF7902` (break `/Game/MainContent/Blueprints/Items/ItemBase/ItemsEquip/Weapons/PenetrationComponent/S_BulletInfo` (`local.CurrentBulletInfo`))) 0.0)
    (`self.DebugSurfaceInfo` _returnvalue_2 "Don't Add Surface Type Decal")
    (`self.HitSpawnFX` (`local.Hit`) _value "/Game/StarterContent/Particles/P_Explosion.P_Explosion")
    (bind (_bsuccess _penetrationlocation) (`self.BulletPenetrationLogic` (`self.GetShotDirection` _hit) _impactpoint _hitactor))
    (if (and (> _returnvalue_4 0.0) _bsuccess)
      (`self.BulletTrace` _penetrationlocation (* (`self.GetShotDirection` (`local.Hit`)) _returnvalue_4) CurrentBulletInfo)
      (else
        (`KismetArrayLibrary.Array_RemoveItem` (`self.BulletsInfo`) (`local.CurrentBulletInfo`))))
    (else
      (`self.DebugSurfaceInfo` _returnvalue_3 "Don't Add Surface Type Last Decal")
      (`self.HitSpawnFX` (`local.Hit`) _value_2 "/Game/StarterContent/Particles/P_Explosion.P_Explosion")
      (`KismetArrayLibrary.Array_RemoveItem` (`self.BulletsInfo`) (`local.CurrentBulletInfo`)))))

(fn `HitSpawnFX`
  (params (Hit :type "HitResult Structure") (DecalBySurface :type "MaterialInterface Object Reference") (EmitterBySurface :type "ParticleSystem Object Reference") (SoundBySurface :type "SoundBase Object Reference"))
  (bind (_bblockinghit _binitialoverlap _time _distance _location _impactpoint _normal _impactnormal) (`GameplayStatics.BreakHitResult` (`local.Hit`)))
  (`self.SpawnDecal` DecalBySurface Hit)
  (`GameplayStatics.SpawnEmitterAtLocation` EmitterBySurface _impactpoint (`KismetMathLibrary.Conv_VectorToRotator` _impactnormal) (0.1 0.1 0.1))
  (`GameplayStatics.PlaySoundAtLocation` SoundBySurface (`.ImpactPoint` (`GameplayStatics.BreakHitResult` (`local.Hit`))) (struct) 1.0 1.0 0.0 null null null null))

(fn `MakeImpulse`
  (params (Hit :type "HitResult Structure (by ref)"))
  (bind (_bblockinghit _binitialoverlap _time _distance _location _impactpoint _normal _impactnormal _physmat _hitactor _hitcomponent _hitbonename _bonename _hititem _elementindex _faceindex _tracestart _traceend) (`GameplayStatics.BreakHitResult` Hit))
  (if _bblockinghit
    (`/Engine/EditorBlueprintResources/StandardMacros.IsValid` _hitcomponent
      (:`Is Valid`
        (if (`SceneComponent.IsSimulatingPhysics` _hitcomponent _bonename)
          (`PrimitiveComponent.AddImpulseAtLocation` _hitcomponent (* (`KismetMathLibrary.GetForwardVector` (`KismetMathLibrary.FindLookAtRotation` _tracestart _traceend)) 4000.0) _impactpoint _bonename))))))

(fn `MakeShot`
  (params (`Muzzle Location` :type "Vector Structure") (`Fire Vector` :type "Vector Structure"))
  (bind _returnvalue (`KismetArrayLibrary.Array_Add` (`self.BulletsInfo`) (make `/Game/MainContent/Blueprints/Items/ItemBase/ItemsEquip/Weapons/PenetrationComponent/S_BulletInfo` (`self.BulletPenetration`) 0.0 (`self.Damage`))))
  (`self.BulletTrace` `Muzzle Location` (* `Fire Vector` (`self.Distance`)) (`|GetArrayItem` (`self.BulletsInfo`) _returnvalue)))

(fn `SpawnDecal`
  (params (DecalMaterial :type "MaterialInterface Object Reference") (Hit :type "HitResult Structure (by ref)"))
  (bind (_bblockinghit _binitialoverlap _time _distance _location _impactpoint _normal _impactnormal _physmat _hitactor _hitcomponent _hitbonename) (`GameplayStatics.BreakHitResult` Hit))
  (bind _returnvalue (`KismetMathLibrary.RandomFloatInRange` 6.0 7.0))
  (`/Engine/EditorBlueprintResources/StandardMacros.IsValid` DecalMaterial
    (:`Is Valid`
      (bind _returnvalue_2 (`GameplayStatics.SpawnDecalAttached` DecalMaterial (`KismetMathLibrary.MakeVector` _returnvalue _returnvalue _returnvalue) _hitcomponent _hitbonename _impactpoint (`KismetMathLibrary.Conv_VectorToRotator` _impactnormal) "KeepWorldPosition" 15.0))
      (`DecalComponent.SetFadeScreenSize` _returnvalue_2 0.002)
      (`SceneComponent.K2_AddRelativeRotation` _returnvalue_2 (`KismetMathLibrary.MakeRotator` (`KismetMathLibrary.RandomFloatInRange` -90.0 90.0)) false false))))