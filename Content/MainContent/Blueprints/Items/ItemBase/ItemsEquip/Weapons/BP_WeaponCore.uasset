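; Base weapon item that handles player firing and reloading, syncing current ammo with its weapon object on equip and unequip.
; Firing is gated by ammo, reload state and a fire-rate delay, then plays effects and spawns bullet actors, several for shotguns.
; Bullets aim from the muzzle toward a screen-center trace, with random spread scaled by player speed.
; Timer-driven reload refills from reserve ammo; aiming only prints debug text.
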(event `self.ReceiveBeginPlay`
  (`parent.ReceiveBeginPlay`))

(event `self.On Equip`
  (`parent.On Equip`)
  (bind _asbp_weapon_object (cast `/Game/MainContent/Blueprints/Items/ItemObjectForInventory/ChildObjects/Weapon/BP_WeaponObject` (`self.ObjectCore`)))
  (set `self.WeaponObject` _asbp_weapon_object)
  (set `self.CurrentAmmo` (`/Game/MainContent/Blueprints/Items/ItemObjectForInventory/ChildObjects/Weapon/BP_WeaponObject.CurrentAmmo` _asbp_weapon_object))
  (add `/Game/MainContent/Blueprints/Player/PlayerCore/BP_Player.TakeDamage` (`self.Player`) (`|CreateDelegate` :!event `StopUseItem`)))

(event `self.UnEquip`
  (set `/Game/MainContent/Blueprints/Items/ItemObjectForInventory/ChildObjects/Weapon/BP_WeaponObject.CurrentAmmo` (`self.CurrentAmmo`) (`self.WeaponObject`)))

(event `self.ReceiveTick`
  (params (DeltaSeconds :type "Float (single-precision)"))
  (`parent.ReceiveTick` DeltaSeconds))

(event `self.StartUse`
  ;[1 1 1] UseItem
  (`self.StartFire`))

(event `Fire`
  ;[1 1 1] Fire
  (`self.CanFire?`)
  (`/Engine/EditorBlueprintResources/StandardMacros.DoOnce` false :!label _label
    (:`Completed`
      (`self.Is Fire?` true)
      (`self.FireLogic`)
      (`KismetSystemLibrary.RetriggerableDelay` (`self.FireRate`))
      (`self.Is Fire?` false)
      (goto _label :!via `Reset`))))

(event `self.StopUse`
  ;[1 1 1] UseItem
  (`self.StopFire`))

(event `StartFire`
  ;[1 1 1] FireLogic
  (`self.CanUse?`)
  (`self.Fire`))

(event `StartReloadLogic`
  ;[1 1 1] ReloadLogic
  (`self.IsCanReload?`
    (:`True`
      (`/Game/MainContent/Blueprints/Player/PlayerCore/BP_Player.PlayPlayerAnimMontage` (`self.Player`) (`self.ReloadAnimMontage`))
      (`self.Is Reload?` true)
      (`self.ReloadTimer` (`self.bIsLoopReload?`) (`self.ReloadTime`)))))

(event `StopFire`
  ;[1 1 1] FireLogic
)

(event `StartReload`
  ;[1 1 1] Reload Weapon
  (`self.StartReloadLogic`))

(event `StopReloadLogic`
  ;[1 1 1] ReloadLogic
  ;;[1 1 1] Либо делать логику перезарядки через аним монтаж(можно ли сделать один нотифай для разных монатжей), либо через timer или delay)(узнать как получить длительность монтажа)
  (`KismetSystemLibrary.PrintString` "Логика перезарядки(добавление патронов)")
  (`self.ReloadLogic`))

(event `StopReload`
  ;[1 1 1] Reload Weapon
  (`self.StopReloadLogic`))

(event `StopUseItem`
  (`self.Is Reload?` false)
  (`KismetSystemLibrary.K2_ClearAndInvalidateTimerHandle` (`self.ReloadTimerHandle`)))

(event `self.StartAction`
  ;[1 1 1] AimLogic
  (`KismetSystemLibrary.PrintString` "Aim"))

(event `self.StopAction`
  ;[1 1 1] AimLogic
  (`KismetSystemLibrary.PrintString` "NoAim"))

(fn `CalculateDirection`
  (returns (DirectionTransform :type "Transform Structure"))
  (bind _muzzlelocation (`self.GetMuzzleInfo`))
  (bind (_x _y) (`KismetMathLibrary.BreakVector2D` (`WidgetLayoutLibrary.GetViewportSize`)))
  (bind (_worldposition _worlddirection) (`GameplayStatics.DeprojectScreenToWorld` (`GameplayStatics.GetPlayerController` 0) (`KismetMathLibrary.MakeVector2D` (/ _x 2.0) (/ _y 2.0))))
  (bind _outhit (`KismetSystemLibrary.LineTraceSingle` :`Start` _worldposition :`End` (+ _worldposition (* _worlddirection 10000.0)) :`TraceChannel` "TraceTypeQuery1" :`DrawDebugType` "ForDuration"))
  (bind (_bblockinghit _binitialoverlap _time _distance _location _impactpoint _normal _impactnormal _physmat _hitactor _hitcomponent _hitbonename _hititem _elementindex _faceindex _tracestart _traceend) (`GameplayStatics.BreakHitResult` _outhit))
  (return (`KismetMathLibrary.MakeTransform` _muzzlelocation (`KismetMathLibrary.FindLookAtRotation` _muzzlelocation (`KismetMathLibrary.SelectVector` _impactpoint _traceend _bblockinghit)))))

(fn `CalculateFinalDirection`
  (params (CalculatedTransform :type "Transform Structure"))
  (returns (FinalTransform :type "Transform Structure"))
  (bind _returnvalue (`KismetMathLibrary.NormalizeToRange` (`/Game/MainContent/Blueprints/Player/PlayerCore/BP_Player.Calculate Character Speed` (`self.Player`)) 0.0 300.0))
  (bind _returnvalue_2 (* (`self.WeaponSpread`) (`KismetMathLibrary.RandomFloatInRange` (* _returnvalue -1.0) _returnvalue)))
  (return (`KismetMathLibrary.MakeTransform` (.location CalculatedTransform) (`KismetMathLibrary.ComposeRotators` (.rotation CalculatedTransform) (`KismetMathLibrary.MakeRotator` (`KismetMathLibrary.RandomFloatInRange` _returnvalue_2) (`KismetMathLibrary.RandomFloatInRange` _returnvalue_2) (`KismetMathLibrary.RandomFloatInRange` _returnvalue_2))))))

(fn `FireLogic`
  (`self.MinusBullet`)
  (`self.PlayAnimMontage` (`self.WeaponAnimMontage`) (`self.CharacterAnimMontage`))
  (`GameplayStatics.PlaySoundAtLocation` (`self.SoundUseItem`) (`self.K2_GetActorLocation`) (struct) 1.0 1.0 0.0 null null null)
  (`self.SpawnFireParticle` (`self.FireParticle`))
  (for _ (range (+ (select `/Game/MainContent/Blueprints/Items/Enumerations/E_ItemType` (`self.ItemType`) :`NewEnumerator0` 4 :`NewEnumerator4` -1 :`NewEnumerator5` -1 :`NewEnumerator7` -1 :`NewEnumerator6` -1) 1))
    (bind _directiontransform (`self.CalculateDirection`))
    (bind _finaltransform (`self.CalculateFinalDirection` _directiontransform))
    (`|SpawnActorFromClass` (`self.WeaponBullet`) _finaltransform "Undefined" "OverrideRootScale" self (`self.Player`))))

(fn `Get Start Ammo`
  (returns (StartAmmo :type Integer))
  (return (`self.StartAmmo`)))

(fn `GetCurrentAmmo`
  (returns (CurrentAmmo :type Integer))
  (return (`self.CurrentAmmo`)))

(fn `GetCurrentMaxAmmo`
  (returns (MaxAmmo :type Integer))
  (return (`self.MaxAmmo`)))

(fn `GetMuzzleInfo`
  (returns (MuzzleLocation :type "Vector Structure"))
  (return (`SceneComponent.GetSocketLocation` (`self.Weapon`) (`self.MuzzleSocketName`))))

(fn `GetStartMaxAmmo`
  (returns (StartMaxAmmo :type Integer))
  (return (`self.StartMaxAmmo`)))

(fn `Is Fire?`
  (params (bFire :type Boolean))
  (set `/Game/MainContent/Blueprints/Player/PlayerCore/BP_Player.bUseItem` bFire (`self.Player`)))

(fn `Is Reload?`
  (params (bReload :type Boolean))
  (set `/Game/MainContent/Blueprints/Player/PlayerCore/BP_Player.bReload` bReload (`self.Player`)))

(fn `MinusBullet`
  (`/Engine/EditorBlueprintResources/StandardMacros.DecrementInt` (`self.CurrentAmmo`)
    (:`  `
      (return))))

(fn `Play Weapon Anim Montage`
  (params (WeaponMontageToPlay :type "AnimMontage Object Reference"))
  (`AnimInstance.Montage_Play` (`SkeletalMeshComponent.GetAnimInstance` (`self.Weapon`)) WeaponMontageToPlay 1.0 "MontageLength" 0.0 true))

(fn `PlayAnimMontage`
  (params (WeaponMontage :type "AnimMontage Object Reference") (CharacterMontage :type "AnimMontage Object Reference"))
  (`/Game/MainContent/Blueprints/Player/PlayerCore/BP_Player.PlayPlayerAnimMontage` (`self.Player`) CharacterMontage))

(fn `Reload`
  (`/Game/MainContent/Blueprints/Player/PlayerCore/BP_Player.PlayPlayerAnimMontage` (`self.Player`) (`self.ReloadAnimMontage`))
  (`self.Is Reload?` true))

(fn `ReloadLogic`
  (locals (LocalCurrentAmmo :type Integer) (LocalMaxAmmo :type Integer))
  (bind _localmaxammo (`local.LocalMaxAmmo`))
  (bind _returnvalue (- (`self.StartAmmo`) (`local.LocalCurrentAmmo`)))
  (bind _returnvalue_2 (> _localmaxammo _returnvalue))
  (set `local.LocalMaxAmmo` (`self.MaxAmmo`))
  (set `local.LocalCurrentAmmo` (`self.CurrentAmmo`))
  (set `self.CurrentAmmo` (`KismetMathLibrary.SelectInt` (`self.StartAmmo`) (+ (`local.LocalMaxAmmo`) (`local.LocalCurrentAmmo`)) _returnvalue_2))
  (set `self.MaxAmmo` (`KismetMathLibrary.SelectInt` (- _localmaxammo _returnvalue) 0 _returnvalue_2))
  (`self.Is Reload?` false))

(fn `ReloadTimer`
  (params (bLoop :type Boolean) (ReloadTime :type "Float (double-precision)"))
  (bind _returnvalue (`KismetSystemLibrary.K2_SetTimerDelegate` (`|CreateDelegate` :!event `StopReload`) ReloadTime bLoop))
  (set `self.ReloadTimerHandle` _returnvalue))

(fn `SpawnFireParticle`
  (params (Particle :type "ParticleSystem Object Reference"))
  (`GameplayStatics.SpawnEmitterAtLocation` Particle (`self.GetMuzzleInfo`) (struct) (0.25 0.25 0.25))
  (return))

(fn `UserConstructionScript`
  (`parent.UserConstructionScript`))