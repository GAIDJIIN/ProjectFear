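; Core Blueprint for equippable consumable items, providing a shared check for whether the item is used up.
; IsSpentAllItems? queries the player's Backpack with IsItemEmpty and, on a false result, runs UnEquipItemLogic and resets the player's animation.
; Its note says it runs alongside the item's logic in an animation timer.
; The event graph holds only disabled placeholder events.
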(fn `IsSpentAllItems?`
  (bind _player (`self.GetPlayer`))
  ;[1 1 1] Вызывать вместе с логикой предмета в таймере с анимацией
  (bind _success (`/Game/MainContent/Blueprints/Player/Components/Inventory/BPC_Inventory.IsItemEmpty?` (`/Game/MainContent/Blueprints/Player/PlayerCore/BP_Player.Backpack` (`self.GetPlayer`)) (`self.GetObject`)))
  (if (not _success)
    (`/Game/MainContent/Blueprints/Player/Components/Inventory/BPC_Inventory.UnEquipItemLogic` (`/Game/MainContent/Blueprints/Player/PlayerCore/BP_Player.Backpack` _player))
    (`/Game/MainContent/Blueprints/Player/PlayerCore/BP_Player.ResetAnimation` _player)))

(fn `UserConstructionScript`
  (`parent.UserConstructionScript`))