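; BP_ItemBase is a base Blueprint for items with a primary use (LMB) and a secondary action (RMB).
; Start and stop events for both inputs forward to matching logic events, which are empty here.
; BeginPlay fires an empty OnEquip event, and getter functions expose the item's ObjectCore and Player references.
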(event `StartUse`
  ;[1 1 1] LMB
  (`self.StartUseLogic`))

(event `StartAction`
  ;[1 1 1] RMB
  (`self.StartActionLogic`))

(event `On Equip`
  ;[1 1 1] OnEquip
)

(event `self.ReceiveBeginPlay`
  ;[1 1 1] OnEquip
  (`self.On Equip`))

(event `StopUse`
  ;[1 1 1] LMB
  (`self.StopUseLogic`))

(event `StopAction`
  ;[1 1 1] RMB
  (`self.StopActionLogic`))

(event `StartUseLogic`
  ;[1 1 1] LogicCore
)

(event `StartActionLogic`
  ;[1 1 1] LogicCore
)

(event `StopUseLogic`
  ;[1 1 1] LogicCore
)

(event `StopActionLogic`
  ;[1 1 1] LogicCore
)

(fn `GetObject`
  (returns (ObjectCore :type "/Game/MainContent/Blueprints/Items/ItemObjectForInventory/BP_ItemObjectCore Object Reference"))
  (return (`self.ObjectCore`)))

(fn `GetPlayer`
  (returns (Player :type "/Game/MainContent/Blueprints/Player/PlayerCore/BP_Player Object Reference"))
  (return (`self.Player`)))

(fn `UserConstructionScript`
  (`parent.UserConstructionScript`))