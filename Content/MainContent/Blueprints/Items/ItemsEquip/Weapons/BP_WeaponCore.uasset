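; Base weapon item for equippable guns, handling use input, single-shot firing with a fire-rate lock, and ammo checks.
; Each shot decrements ammo, plays sound and muzzle particles, then spawns bullet actors, several for shotguns.
; Bullets leave the muzzle socket toward a screen-center trace hit, with random spread scaled by character velocity.
; Reload only plays a player montage and prints; aiming, ammo refill and the fire montage function are stubs.
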(event `self.ReceiveBeginPlay`
  (`parent.ReceiveBeginPlay`))

(event `self.StartUse`
  ;[1 1 1] UseItem
  (`self.StartFire`))

(event `Fire`
  ;[1 1 1] Fire
  (`self.CanFire?`)
  (switch `/Game/MainContent/Blueprints/Items/Enumerations/EFireMode` (`self.FireMode`)
    (:`NewEnumerator0`
      (`/Engine/EditorBlueprintResources/StandardMacros.DoOnce` false :!label _label
        (:`Completed`
          (`self.Is Fire?` true)
          (`self.FireLogic`)
          (`KismetSystemLibrary.RetriggerableDelay` (`self.FireRate`))
          (`self.Is Fire?` false)
          (goto _label :!via `Reset`))))))

(event `self.StopUse`
  ;[1 1 1] UseItem
  (`self.StopFire`))

(event `StartFire`
  ;[1 1 1] FireLogic
  (`self.CanUse?`)
  (`self.Fire`))

(event `StartReload`
  ;[1 1 1] ReloadLogic
  (`KismetSystemLibrary.PrintString` "Проверка патронов")
  (`/Game/MainContent/Blueprints/Player/PlayerCore/BP_Player.PlayPlayerAnimMontage` (`self.GetPlayer`) (`self.ReloadAnimMontage`)))

(event `StopFire`
  ;[1 1 1] FireLogic
)

(event `self.StartAction`
  ;[1 1 1] AimLogic
  (`KismetSystemLibrary.PrintString` "Aim"))

(event `StopReload`
  ;[1 1 1] ReloadLogic
  (`KismetSystemLibrary.PrintString` "Логика перезарядки(добавление патронов)"))

(event `self.StopAction`
  ;[1 1 1] AimLogic
  (`KismetSystemLibrary.PrintString` "NoAim"))

(fn `CalculateCharacterVelocity`
  (returns (CharacterVelocity :type "Float (double-precision)"))
  (return (`KismetMathLibrary.VSize` (`self.GetVelocity` (`self.Character`)))))

(fn `CalculateDirection`
  (returns (DirectionTransform :type "Transform Structure"))
  (bind _muzzlelocation (`self.GetMuzzleInfo`))
  (bind (_x _y) (`KismetMathLibrary.BreakVector2D` (`WidgetLayoutLibrary.GetViewportSize`)))
  (bind (_worldposition _worlddirection) (`GameplayStatics.DeprojectScreenToWorld` (`GameplayStatics.GetPlayerController` 0) (`KismetMathLibrary.MakeVector2D` (/ _x 2.0) (/ _y 2.0))))
  (bind _outhit (`KismetSystemLibrary.LineTraceSingle` :`Start` _worldposition :`End` (+ _worldposition (* _worlddirection 10000.0)) :`TraceChannel` "TraceTypeQuery1" :`DrawDebugType` "ForDuration"))
  (bind (_bblockinghit _binitialoverlap _time _distance _location _impactpoint _normal _impactnormal _physmat _hitactor _hitcomponent _hitbonename _hititem _elementindex _faceindex _tracestart _traceend) (`GameplayStatics.BreakHitResult` _outhit))
  (return (`KismetMathLibrary.MakeTransform` _muzzlelocation (`KismetMathLibrary.FindLookAtRotation` _muzzlelocation (`KismetMathLibrary.SelectVector` _impactpoint _traceend _bblockinghit)))))

(fn `CalculateFinalDirection`
  (params (CalculatedTransform :type "Transform Structure"))
  (returns (FinalTransform :type "Transform Structure"))
  (bind _returnvalue (`KismetMathLibrary.NormalizeToRange` (`self.CalculateCharacterVelocity`) 0.0 300.0))
  (bind _returnvalue_2 (* (`self.WeaponSpread`) (`KismetMathLibrary.RandomFloatInRange` (* _returnvalue -1.0) _returnvalue)))
  (return (`KismetMathLibrary.MakeTransform` (.location CalculatedTransform) (`KismetMathLibrary.ComposeRotators` (.rotation CalculatedTransform) (`KismetMathLibrary.MakeRotator` (`KismetMathLibrary.RandomFloatInRange` _returnvalue_2) (`KismetMathLibrary.RandomFloatInRange` _returnvalue_2) (`KismetMathLibrary.RandomFloatInRange` _returnvalue_2))))))

(fn `FireLogic`
  (`self.MinusBullet`)
  (`self.PlayAnimMontage` (`self.WeaponAnimMontage`) (`self.CharacterAnimMontage`))
  (`GameplayStatics.PlaySoundAtLocation` (`self.WeaponSound`) (`self.K2_GetActorLocation`) (struct) 1.0 1.0 0.0 null null null)
  (`self.SpawnFireParticle` (`self.FireParticle`))
  (for _ (range (+ (select `/Game/MainContent/Blueprints/Items/Enumerations/EItemType` (`self.ItemType`) :`NewEnumerator0` 5 :`NewEnumerator4` -1 :`NewEnumerator5` -1 :`NewEnumerator6` -1 :`NewEnumerator7` -1) 1))
    (bind _directiontransform (`self.CalculateDirection`))
    (bind _finaltransform (`self.CalculateFinalDirection` _directiontransform))
    (`|SpawnActorFromClass` (`self.WeaponBullet`) _finaltransform "Undefined" "OverrideRootScale" self (`self.Character`))))

(fn `GetCurrentAmmo`
  (returns (CurrentAmmo :type Integer))
  (return (`self.CurrentAmmo`)))

(fn `GetCurrentMaxAmmo`
  (returns (MaxAmmo :type Integer))
  (return (`self.MaxAmmo`)))

(fn `GetMuzzleInfo`
  (returns (MuzzleLocation :type "Vector Structure"))
  (return (`SceneComponent.GetSocketLocation` (`self.Weapon`) (`self.MuzzleName`))))

(fn `Is Fire?`
  (params (bFire :type Boolean))
  (set `/Game/MainContent/Blueprints/Player/PlayerCore/BP_Player.bUseItem` bFire (`self.GetPlayer`)))

(fn `MinusBullet`
  (`/Engine/EditorBlueprintResources/StandardMacros.DecrementInt` (`self.CurrentAmmo`)
    (:`  `
      (return))))

(fn `PlayAnimMontage`
  (params (WeaponMontage :type "AnimMontage Object Reference") (CharacterMontage :type "AnimMontage Object Reference")))

(fn `PlayWeaponAnimMontage`
  (params (WeaponMontageToPlay :type "AnimMontage Object Reference"))
  (`AnimInstance.Montage_Play` (`SkeletalMeshComponent.GetAnimInstance` (`self.Weapon`)) WeaponMontageToPlay 1.0 "MontageLength" 0.0 true))

(fn `SpawnFireParticle`
  (params (Particle :type "ParticleSystem Object Reference"))
  (`GameplayStatics.SpawnEmitterAtLocation` Particle (`self.GetMuzzleInfo`) (struct) (0.25 0.25 0.25))
  (return))

(fn `UserConstructionScript`
  (`parent.UserConstructionScript`))