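; BP_WeaponCore is a weapon actor, apparently a base class, that fires projectiles on use and exposes ammo counts.
; Single fire mode, the only one wired, gates shots by FireRate and flags BP_Player's UseItem.
; FireLogic plays sound and muzzle particles, then spawns ItemType-dependent bullets aimed via screen-centre trace, with random spread scaled by character speed.
; Ammo decrement, montage playback and StopFire are empty stubs; trace drawing and rotation printing remain enabled.
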(event `self.ReceiveBeginPlay`
  (`parent.ReceiveBeginPlay`))

(event `self.StartUse`
  (`self.StartFire`))

(event `self.StopUse`
  (`self.StopFire`))

(event `StartFire`
  (`self.Fire`))

(event `Fire`
  (switch `/Game/MainContent/Blueprints/Items/Enumerations/EFireMode` (`self.FireMode`)
    (:`NewEnumerator0`
      (`/Engine/EditorBlueprintResources/StandardMacros.DoOnce` false :!label _label
        (:`Completed`
          (`self.Is Fire?` true)
          (`self.FireLogic`)
          (`KismetSystemLibrary.RetriggerableDelay` (`self.FireRate`))
          (`self.Is Fire?` false)
          (goto _label :!via `Reset`))))))

(event `StopFire`)

(fn `CalculateCharacterVelocity`
  (returns (CharacterVelocity :type "Float (double-precision)"))
  (return (`KismetMathLibrary.VSize` (`self.GetVelocity` (`self.Character`)))))

(fn `CalculateDirection`
  (returns (DirectionTransform :type "Transform Structure"))
  (bind _muzzlelocation (`self.GetMuzzleInfo`))
  (bind (_x _y) (`KismetMathLibrary.BreakVector2D` (`WidgetLayoutLibrary.GetViewportSize`)))
  (bind (_worldposition _worlddirection) (`GameplayStatics.DeprojectScreenToWorld` (`GameplayStatics.GetPlayerController` 0) (`KismetMathLibrary.MakeVector2D` (/ _x 2.0) (/ _y 2.0))))
  (bind _outhit (`KismetSystemLibrary.LineTraceSingle` :`Start` _worldposition :`End` (+ _worldposition (* _worlddirection 10000.0)) :`TraceChannel` "TraceTypeQuery1" :`DrawDebugType` "ForDuration"))
  (bind (_bblockinghit _binitialoverlap _time _distance _location _impactpoint _normal _impactnormal _physmat _hitactor _hitcomponent _hitbonename _hititem _elementindex _faceindex _tracestart _traceend) (`GameplayStatics.BreakHitResult` _outhit))
  (return (`KismetMathLibrary.MakeTransform` _muzzlelocation (`KismetMathLibrary.FindLookAtRotation` _muzzlelocation (`KismetMathLibrary.SelectVector` _impactpoint _traceend _bblockinghit)))))

(fn `CalculateFinalDirection`
  (params (CalculatedTransform :type "Transform Structure"))
  (returns (FinalTransform :type "Transform Structure"))
  (bind _returnvalue (`KismetMathLibrary.NormalizeToRange` (`self.CalculateCharacterVelocity`) 0.0 300.0))
  (bind _returnvalue_2 (* (`self.WeaponSpread`) (`KismetMathLibrary.RandomFloatInRange` (* _returnvalue -1.0) _returnvalue)))
  (bind _returnvalue_3 (`KismetMathLibrary.ComposeRotators` (.rotation CalculatedTransform) (`KismetMathLibrary.MakeRotator` (`KismetMathLibrary.RandomFloatInRange` _returnvalue_2) (`KismetMathLibrary.RandomFloatInRange` _returnvalue_2) (`KismetMathLibrary.RandomFloatInRange` _returnvalue_2))))
  (`KismetSystemLibrary.PrintString` (`KismetStringLibrary.Conv_RotatorToString` _returnvalue_3))
  (return (`KismetMathLibrary.MakeTransform` (.location CalculatedTransform) _returnvalue_3)))

(fn `FireLogic`
  (`self.MinusBullet`)
  (`self.PlayAnimMontage` (`self.WeaponAnimMontage`) (`self.CharacterAnimMontage`))
  (`GameplayStatics.PlaySoundAtLocation` (`self.WeaponSound`) (`self.K2_GetActorLocation`) (struct) 1.0 1.0 0.0 null null null)
  (`self.SpawnFireParticle` (`self.FireParticle`))
  (for _ (range (+ (select `/Game/MainContent/Blueprints/Items/Enumerations/EItemType` (`self.ItemType`) :`NewEnumerator0` 5 :`NewEnumerator1` 1 :`NewEnumerator2` 1 :`NewEnumerator3` 1) 1))
    (bind _directiontransform (`self.CalculateDirection`))
    (bind _finaltransform (`self.CalculateFinalDirection` _directiontransform))
    (`|SpawnActorFromClass` (`self.WeaponBullet`) _finaltransform "Undefined" "OverrideRootScale" self (`self.Character`))))

(fn `GetCurrentAmmo`
  (returns (CurrentAmmo :type Integer))
  (return (`self.CurrentAmmo`)))

(fn `GetCurrentMaxAmmo`
  (returns (MaxAmmo :type Integer))
  (return (`self.MaxAmmo`)))

(fn `GetMuzzleInfo`
  (returns (MuzzleLocation :type "Vector Structure"))
  (return (`SceneComponent.GetSocketLocation` (`self.Weapon`) (`self.MuzzleName`))))

(fn `Is Fire?`
  (params (bFire :type Boolean))
  (set `/Game/MainContent/Blueprints/Player/PlayerCore/BP_Player.bUseItem` bFire (cast `/Game/MainContent/Blueprints/Player/PlayerCore/BP_Player` (`self.Character`) :!pure true)))

(fn `MinusBullet`)

(fn `PlayAnimMontage`
  (params (WeaponMontage :type "AnimMontage Object Reference") (CharacterMontage :type "AnimMontage Object Reference")))

(fn `SpawnFireParticle`
  (params (Particle :type "ParticleSystem Object Reference"))
  (`GameplayStatics.SpawnEmitterAtLocation` Particle (`self.GetMuzzleInfo`) (struct) (0.25 0.25 0.25))
  (return))

(fn `UserConstructionScript`
  (`parent.UserConstructionScript`)
  (set `self.CurrentAmmo` (`self.StartAmmo`))
  (set `self.MaxAmmo` (`self.StartMaxAmmo`)))