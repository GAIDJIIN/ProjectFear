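; BP_PickUpCore is a world item pickup that, on interaction, offers its item to the player's Backpack, then plays a sound and destroys itself if accepted.
; It uses an existing item object or lazily constructs one from its data table row and quantity.
; The construction script sets the mesh from either source.
; On first hit, it lets Pawns overlap until clear of its instigator, then blocks them.
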(event `/Game/MainContent/Blueprints/Items/Interfaces/BPI_Interact.StartInteract`
  (params (Player :type "/Game/MainContent/Blueprints/Player/PlayerCore/BP_Player Object Reference"))
  ;[1 1 1] Interfaces
  (`self.StartPickUpLogic` Player))

(event `StartPickUpLogic`
  (params (Player :type "/Game/MainContent/Blueprints/Player/PlayerCore/BP_Player Object Reference"))
  ;[1 1 1] LogicInteract
  (bind _itemobject (`self.IsValidObject`))
  (bind _success (`/Game/MainContent/Blueprints/Player/Components/Inventory/BPC_Inventory.CanAddItem?` (`/Game/MainContent/Blueprints/Player/PlayerCore/BP_Player.Backpack` Player) _itemobject))
  (if _success
    (`GameplayStatics.PlaySoundAtLocation` (`self.SoundPickUp`) (`self.K2_GetActorLocation`) (struct) 1.0 1.0 0.0 null null null null)
    (`self.K2_DestroyActor`)))

(event `self.ReceiveBeginPlay`
  ;[1 1 1] Comment
  (add `self.OnActorHit` (delegate `HitFunction`)))

(event `HitFunction` :!signature `self.OnActorHit`
  (params (SelfActor :type "Actor Object Reference") (OtherActor :type "Actor Object Reference") (NormalImpulse :type "Vector Structure") (Hit :type "HitResult Structure (by ref)"))
  ;[1 1 1] Comment
  (`/Engine/EditorBlueprintResources/StandardMacros.DoOnce` false
    (:`Completed`
      (`/Engine/EditorBlueprintResources/StandardMacros.IsValid` (`self.GetInstigator`)
        (:`Is Valid`
          (`PrimitiveComponent.SetCollisionResponseToChannel` (`self.ItemPickUp`) "ECC_Pawn" "ECR_Overlap")
          (if (not (`PrimitiveComponent.IsOverlappingActor` (`self.ItemPickUp`) (`self.GetInstigator`)))
            (`self.SetBlock` :!label _label)))
        (:`Is Not Valid`
          (`self.SetBlock`))))))

(event `self.ItemPickUp.OnComponentEndOverlap`
  (params (OverlappedComponent :type "PrimitiveComponent Object Reference") (OtherActor :type "Actor Object Reference") (OtherComp :type "PrimitiveComponent Object Reference") (OtherBodyIndex :type Integer))
  ;[1 1 1] Comment
  (if (== OtherActor (`self.GetInstigator`))
    (goto _label)))

(fn `GetObject`
  (returns (ObjectItem :type "/Game/MainContent/Blueprints/Items/ItemObjectForInventory/BP_ItemObjectCore Object Reference"))
  (return (`self.ObjectItem`)))

(fn `IsValidObject`
  (returns (ItemObject :type "/Game/MainContent/Blueprints/Items/ItemObjectForInventory/BP_ItemObjectCore Object Reference"))
  (`/Engine/EditorBlueprintResources/StandardMacros.IsValid` (`self.ObjectItem`)
    (:`Is Valid`
      (return (`self.ObjectItem`)))
    (:`Is Not Valid`
      (bind _itemobject (`self.OnPickUp`))
      (bind _output_get (set `self.ObjectItem` _itemobject))
      (return _output_get))))

(fn `OnPickUp`
  (returns (ItemObject :type "/Game/MainContent/Blueprints/Items/ItemObjectForInventory/BP_ItemObjectCore Object Reference"))
  (bind _returnvalue (`|GenericCreateObject` self "/Game/MainContent/Blueprints/Items/ItemObjectForInventory/BP_ItemObjectCore.BP_ItemObjectCore_C" (`self.Quantity`) (`self.ItemDataTable`)))
  (return _returnvalue))

(fn `SetBlock`
  (bind _itempickup (`self.ItemPickUp`))
  (`PrimitiveComponent.SetCollisionResponseToChannel` _itempickup "ECC_Pawn" "ECR_Block")
  (set `PrimitiveComponent.bGenerateOverlapEvents` false _itempickup)
  (remove `self.OnActorHit` (`|CreateDelegate` :!event `HitFunction`)))

(fn `UserConstructionScript`
  (bind (_datatable _rowname) (break `DataTableRowHandle` (`self.ItemDataTable`)))
  (`/Engine/EditorBlueprintResources/StandardMacros.IsValid` (`self.ObjectItem`)
    (:`Is Valid`
      (`StaticMeshComponent.SetStaticMesh` (`self.ItemPickUp`) (`.Model_40_223642B14823BCB76318F0BBEA27ECC4` (break `/Game/MainContent/Blueprints/Player/Components/Inventory/S_Item` (`/Game/MainContent/Blueprints/Items/ItemObjectForInventory/BP_ItemObjectCore.GetItemStructure` (`self.ObjectItem`))))))
    (:`Is Not Valid`
      (bind _returnvalue (`|GetDataTableRow` _datatable _rowname)
        (:`then`
          (bind ((`MaxStuckSize_10_1AD33E5548CCE857DFD4ACA09E8B119C` _maxstucksize) (`Model_40_223642B14823BCB76318F0BBEA27ECC4` _model)) (break `/Game/MainContent/Blueprints/Player/Components/Inventory/S_Item` _returnvalue))
          (`StaticMeshComponent.SetStaticMesh` (`self.ItemPickUp`) _model)
          (set `self.Quantity` (`KismetMathLibrary.Min` (`self.Quantity`) _maxstucksize)))))))