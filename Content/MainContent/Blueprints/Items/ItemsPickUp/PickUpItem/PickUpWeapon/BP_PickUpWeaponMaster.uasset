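; BP_PickUpWeaponMaster is, by its name, the base Blueprint for weapon pickups, supplying the item object produced when a weapon is picked up.
; OnPickUp constructs a BP_WeaponObject with the pickup as Outer, passes in CurrentAmmo, Quantity and ItemDataTable (as ItemID), and returns it.
; BeginPlay and the construction script only call the parent, while overlap and Tick are disabled stubs.
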(event `self.ReceiveBeginPlay`
  (`parent.ReceiveBeginPlay`))

(fn `OnPickUp`
  (returns (ItemObject :type "/Game/MainContent/Blueprints/Items/ItemObjectForInventory/BP_ItemObjectCore Object Reference"))
  (bind _returnvalue (`|GenericCreateObject` "/Game/MainContent/Blueprints/Items/ItemObjectForInventory/ChildObjects/Weapon/BP_WeaponObject.BP_WeaponObject_C" self (`self.CurrentAmmo`) (`self.Quantity`) (`self.ItemDataTable`)))
  (return _returnvalue))

(fn `UserConstructionScript`
  (`parent.UserConstructionScript`))