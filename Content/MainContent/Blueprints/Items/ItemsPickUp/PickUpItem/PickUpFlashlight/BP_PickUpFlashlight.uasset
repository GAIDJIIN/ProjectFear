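; World pickup actor for the flashlight item, which can show as switched on or off.
; The construction script takes the on state from its flashlight item object if valid, otherwise from its own IsEnable.
; EnableLight applies that state to the light's visibility and the mesh's "Enable" material parameter.
; OnPickUp constructs and returns a BP_FlashLightObject carrying the on state, quantity and item ID.
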(event `self.ReceiveTick`
  (params (DeltaSeconds :type "Float (single-precision)"))
  (`parent.ReceiveTick` DeltaSeconds))

(fn `EnableLight`
  (params (`IsEnable?` :type Boolean))
  (`SceneComponent.SetVisibility` (`self.Light`) `IsEnable?` false)
  (`MeshComponent.SetScalarParameterValueOnMaterials` (`self.ItemPickUp`) "Enable" (`KismetMathLibrary.SelectFloat` 3.0 0.0 `IsEnable?`)))

(fn `OnPickUp`
  (returns (ItemObject :type "/Game/MainContent/Blueprints/Items/ItemObjectForInventory/BP_ItemObjectCore Object Reference"))
  (bind _returnvalue (`|GenericCreateObject` self "/Game/MainContent/Blueprints/Items/ItemObjectForInventory/ChildObjects/BP_FlashLightObject.BP_FlashLightObject_C" (`self.bIsEnable?`) (`self.Quantity`) (`self.ItemDataTable`)))
  (return _returnvalue))

(fn `UserConstructionScript`
  (bind _objectitem (`self.ObjectItem`))
  (`parent.UserConstructionScript`)
  (`/Engine/EditorBlueprintResources/StandardMacros.IsValid` _objectitem
    (:`Is Valid`
      (`self.EnableLight` (`/Game/MainContent/Blueprints/Items/ItemObjectForInventory/ChildObjects/BP_FlashLightObject.IsEnable?` (cast `/Game/MainContent/Blueprints/Items/ItemObjectForInventory/ChildObjects/BP_FlashLightObject` _objectitem :!pure true))))
    (:`Is Not Valid`
      (`self.EnableLight` (`self.bIsEnable?`)))))