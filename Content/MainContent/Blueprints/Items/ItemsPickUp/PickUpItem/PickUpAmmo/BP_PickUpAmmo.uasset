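; BP_PickUpAmmo is the ammo pickup item Blueprint, a child class that leaves pickup behavior to its parent.
; Its Construction Function override passes the item struct's fields and the quantity straight to the parent implementation.
; The construction script only calls the parent, and the event graph holds only disabled default events, so the class adds no logic of its own.
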(fn `Construction Function`
  (params (ItemStruct :type "/Game/MainContent/Blueprints/Player/Components/Inventory/Item_Structure Structure") (`Item Quantity` :type Integer))
  (bind (_name _description _icon _itemclass _maxstucksize _model _isstackable_ _itemtype _pickupitemclass) (break `/Game/MainContent/Blueprints/Player/Components/Inventory/Item_Structure` ItemStruct))
  (bind ((`Name_25_E762B8E7451283CD22642B8F7160541E` _name_2) (`Description_4_C911F9224FF4D2108DA869A9FDE18B66` _description_2) (`Icon_17_1694CBC344AD7037457699A27EF0FF98` _icon_2) (`Model_28_223642B14823BCB76318F0BBEA27ECC4` _model_2)) (break `/Game/MainContent/Blueprints/Player/Components/Inventory/Item_Structure` (`self.ItemStruct`)))
  (`parent.Construction Function` (make `/Game/MainContent/Blueprints/Player/Components/Inventory/Item_Structure` _name_2 _description_2 _icon_2 _itemclass _maxstucksize _model_2 _isstackable_ _itemtype _pickupitemclass) `Item Quantity`))

(fn `UserConstructionScript`
  (`parent.UserConstructionScript`))