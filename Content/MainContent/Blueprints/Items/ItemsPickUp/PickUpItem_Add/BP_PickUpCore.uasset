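; Base pickup item actor that configures its mesh and item data from a Data Table row picked through a row handle.
; The Construction Script applies the row's model to the ItemPickUp mesh and fills ItemStruct, with DefaultName choosing between table and existing name and description.
; The event graph holds only disabled stubs, and an older hardcoded per-ItemType setup of classes, meshes and flags remains disconnected.
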(fn `UserConstructionScript`
  (bind _bdefaultname_ (`self.bDefaultName?`))
  (bind (_datatable _rowname) (break `DataTableRowHandle` (`self.DataTableRow`)))
  (bind (_name _description) (break `/Game/MainContent/Blueprints/Player/Components/Inventory/Item_Structure` (`self.ItemStruct`)))
  (`parent.UserConstructionScript`)
  (bind _returnvalue (`|GetDataTableRow` _datatable _rowname)
    (:`then`
      (bind (_name_2 _description_2 _icon _itemclass _maxstucksize _model _isstackable_ _itemtype) (break `/Game/MainContent/Blueprints/Player/Components/Inventory/Item_Structure` _returnvalue))
      (`StaticMeshComponent.SetStaticMesh` (`self.ItemPickUp`) _model)
      (set `self.ItemStruct` (make `/Game/MainContent/Blueprints/Player/Components/Inventory/Item_Structure` (select `bool` _bdefaultname_ :`false` _name :`true` _name_2) (select `bool` _bdefaultname_ :`false` _description :`true` _description_2) _icon _itemclass _maxstucksize _model _isstackable_ _itemtype)))))