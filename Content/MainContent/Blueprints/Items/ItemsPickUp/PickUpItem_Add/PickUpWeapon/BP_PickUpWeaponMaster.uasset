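; Base weapon pickup Blueprint that carries current and max ammo values for the weapon class referenced by its item struct.
; The construction script reads that class's defaults as a BP_WeaponCore and caps both values at its starting ammo and starting max ammo.
; BeginPlay only calls the parent, and the overlap and tick events are disabled stubs.
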(event `self.ReceiveBeginPlay`
  (`parent.ReceiveBeginPlay`))

(fn `UserConstructionScript`
  (bind (_muzzlesocketname _startammo _startmaxammo) (defaults `Object` (castclass `/Game/MainContent/Blueprints/Items/ItemBase/ItemsEquip/Weapons/BP_WeaponCore` (`.ItemClass_29_E3D0B3EC41DC869E4E07A5B343C5A2E3` (break `/Game/MainContent/Blueprints/Player/Components/Inventory/Item_Structure` (`self.ItemStruct`))) :!pure true)))
  (`parent.UserConstructionScript`)
  (set `self.CurrentAmmo` (`KismetMathLibrary.Min` _startammo (`self.CurrentAmmo`)))
  (set `self.CurrentMaxAmmo` (`KismetMathLibrary.Min` _startmaxammo (`self.CurrentMaxAmmo`))))