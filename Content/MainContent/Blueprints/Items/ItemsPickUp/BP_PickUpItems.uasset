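; BP_PickUpItems is an interactable item Blueprint, named for pickups, that currently holds only the skeleton of the interaction flow.
; StartInteract and StopInteract forward to the custom events StartInter and StopInter.
; StartInter casts the interacting player to BP_Player, while StopInter is empty, so no pickup logic runs in this graph.
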(event `/Game/MainContent/Blueprints/Items/Interfaces/BPI_Interact.StartInteract`
  (params (Player :type "/Game/MainContent/Blueprints/Player/PlayerCore/BP_Player Object Reference"))
  (`self.StartInter` Player))

(event `/Game/MainContent/Blueprints/Items/Interfaces/BPI_Interact.StopInteract`
  (`self.StopInter`))

(event `StartInter`
  (params (PlayerReference :type "/Game/MainContent/Blueprints/Core/BP_CharacterCore Object Reference"))
  (set `self.Character` (cast `/Game/MainContent/Blueprints/Player/PlayerCore/BP_Player` PlayerReference :!pure true)))

(event `StopInter`)

(fn `UserConstructionScript`
  (`parent.UserConstructionScript`))