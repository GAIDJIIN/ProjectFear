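; BP_Door is an interactable environment door that can require a key item matched by data table row handle.
; BeginPlay marks it locked if a KeyID is set; using the matching held item consumes one, updates the player's backpack and unlocks it without opening.
; Once unlocked, a FlipFlop plays or reverses a timeline that rotates the door's yaw.
; Metal sounds mark opening, unlocking, failed attempts and closing.
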(event `self.ReceiveBeginPlay`
  (if (== (`.RowName` (break `DataTableRowHandle` (`self.KeyID`))) "None")
    (set `self.NeedKey?` false)
    (else
      (set `self.NeedKey?` true))))

(event `self.StartInteractLogic`
  (params (Player :type "/Game/MainContent/Blueprints/Player/PlayerCore/BP_Player Object Reference") (HitComponent :type "PrimitiveComponent Object Reference"))
  (bind _iteminhand (`/Game/MainContent/Blueprints/Player/PlayerCore/BP_Player.GetCurrentItem` Player))
  (bind _backpack (`/Game/MainContent/Blueprints/Player/PlayerCore/BP_Player.Backpack` Player))
  (bind _objectcore (`/Game/MainContent/Blueprints/Items/ItemBase/BP_ItemBase.GetObject` _iteminhand))
  (if (`self.NeedKey?`)
    (`/Engine/EditorBlueprintResources/StandardMacros.IsValid` _iteminhand
      (:`Is Valid`
        (if (`/Game/MainContent/Blueprints/ServiceLibrary/ServiceFunctions.EqualDataTableRowHandle` (`/Game/MainContent/Blueprints/Items/ItemObjectForInventory/BP_ItemObjectCore.GetItemID` _objectcore) (`self.KeyID`))
          (`/Engine/EditorBlueprintResources/StandardMacros.DecrementInt` (`/Game/MainContent/Blueprints/Items/ItemObjectForInventory/BP_ItemObjectCore.Quantity` _objectcore)
            (:`  `
              (`/Game/MainContent/Blueprints/Player/Components/Inventory/BPC_Inventory.IsItemEmpty?` _backpack _objectcore)
              (`/Game/MainContent/Blueprints/Player/Components/Inventory/BPC_Inventory.UnEquipItemLogic` _backpack)
              (set `self.NeedKey?` false)
              (`GameplayStatics.PlaySoundAtLocation` "/Game/MainContent/Blueprints/TestLogic/Door/Sounds/MetalDoor_Open.MetalDoor_Open" (`self.K2_GetActorLocation`) (struct) 1.0 1.0 0.0 null null null null)))
          (else
            (`GameplayStatics.PlaySoundAtLocation` "/Game/MainContent/Blueprints/TestLogic/Door/Sounds/MetalDoor_Close.MetalDoor_Close" (`self.K2_GetActorLocation`) (struct) 1.0 1.0 0.0 null null null null :!label _label))))
      (:`Is Not Valid`
        (goto _label)))
    (else
      (`/Engine/EditorBlueprintResources/StandardMacros.FlipFlop`
        (:`A`
          (`GameplayStatics.PlaySoundAtLocation` "/Game/MainContent/Blueprints/TestLogic/Door/Sounds/MetalDoor_Open.MetalDoor_Open" (`self.K2_GetActorLocation`) (struct) 1.0 1.0 0.0 null null null null)
          (bind (_direction _opendoor) (`Timeline|TimeDoor` :!label _label_2)
            (:`Update`
              (`SceneComponent.K2_SetRelativeRotation` (`self.Door`) (`KismetMathLibrary.MakeRotator` 0.0 0.0 _opendoor) false false))
            (:`Finished`
              (switch `ETimelineDirection` _direction
                (:`Backward`
                  (`GameplayStatics.PlaySoundAtLocation` "/Game/MainContent/Blueprints/TestLogic/Door/Sounds/MetalDoor_Close.MetalDoor_Close" (`self.K2_GetActorLocation`) (struct) 1.0 1.0 0.0 null null null null))))))
        (:`B`
          (goto _label_2 :!via `Reverse`))))))

(fn `UserConstructionScript`
  (`parent.UserConstructionScript`))