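; Flashlight component for pickup items that switches a light on and off and drains its battery.
; InitializeProperties stores the owner-supplied mesh and light source, which ToggleLight drives through light visibility and a material scalar for the glow.
; TurnOnStart toggles only with charge left and starts a looping WasteEnergy timer by function name when switching on.
; WasteEnergy decrements charge, clearing the timer and shutting the light off only at empty.
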(fn `InitializeProperties`
  (params (FlashlightMesh :type "StaticMeshComponent Object Reference") (FlashlightSource :type "SpotLightComponent Object Reference"))
  (set `self.FlashlightMesh` FlashlightMesh)
  (set `self.FlashlightSource` FlashlightSource))

(fn `ToggleLight`
  (params (`On&Off` :type Boolean))
  (`SceneComponent.SetVisibility` (`self.FlashlightSource`) `On&Off` false)
  (`MeshComponent.SetScalarParameterValueOnMaterials` (`self.FlashlightMesh`) (`self.LightSourceMaterialName`) (`KismetMathLibrary.SelectFloat` 3.0 0.0 `On&Off`)))

(fn `TurnOnStart`
  (params (BatteryEnergy :type "Integer (by ref)") (`On&Off` :type "Boolean (by ref)"))
  (if (> BatteryEnergy 0)
    (`self.ToggleLight` `On&Off`)
    (if `On&Off`
      (bind _returnvalue (`KismetSystemLibrary.K2_SetTimer` null "WasteEnergy" 0.5 true))
      (set `self.WasteBatteryEnergyTimer` _returnvalue))))

(fn `WasteEnergy`
  (params (BatteryEnergy :type "Integer (by ref)") (`IsEnable?` :type "Boolean (by ref)"))
  (bind _isenable_ (`local.IsEnable?`))
  (`KismetSystemLibrary.PrintString` (`KismetStringLibrary.Conv_IntToString` BatteryEnergy))
  (if (> BatteryEnergy 0)
    (`/Engine/EditorBlueprintResources/StandardMacros.DecrementInt` (`local.BatteryEnergy`))
    (else
      (`KismetSystemLibrary.K2_ClearAndInvalidateTimerHandle` (`self.WasteBatteryEnergyTimer`))
      (`|VariableSetRef` _isenable_)
      (`self.ToggleLight` _isenable_))))